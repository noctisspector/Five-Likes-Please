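; DebugCurve_BP is a debug actor that visualizes a float curve as a line of colored points in the world.
; On BeginPlay it draws long-lasting debug points along world X from its location, spaced by Inc.
; Each point samples Curve at its offset divided by 3000.
; The value, normalized to the curve's value range, shades the point from red to white rather than changing its height.
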(event `self.ReceiveBeginPlay`
  (bind _curve (`self.Curve`))
  (bind (_minvalue _maxvalue) (`CurveBase.GetValueRange` _curve))
  (for _index (range 101)
    (bind _returnvalue (* _index (`self.Inc`)))
    (bind _returnvalue_2 (`KismetMathLibrary.MapRangeClamped` (`CurveFloat.GetFloatValue` _curve (/ _returnvalue 3000.0)) _minvalue _maxvalue 0.0 1.0))
    (`KismetSystemLibrary.DrawDebugPoint` (+ (`self.K2_GetActorLocation`) (`KismetMathLibrary.MakeVector` _returnvalue)) 5.0 (make `LinearColor` 1.0 _returnvalue_2 _returnvalue_2 1.0) 999999995904.0)))

(fn `UserConstructionScript`)