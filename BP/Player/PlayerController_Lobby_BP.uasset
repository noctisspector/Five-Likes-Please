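; Lobby player controller that moves the player between the main menu lobby and the firing range.
; Entering the range unpossesses and destroys the lobby pawn, then calls RespawnServer with the killcam disabled.
; Returning spawns and possesses a new lobby pawn at the first PlayerStart found, with its widget skipped.
; It then opens the loadout screen in main-menu mode through the game instance, with cursor and UI-only input.
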(event `Go to Firing Range`
  (bind _asplayer_lobby_bp (cast `/Game/BP/Player/PlayerLobby_BP` (`GameplayStatics.GetPlayerPawn` 0)))
  (bind _output_get (set `self.Last Player` _asplayer_lobby_bp))
  (`self.UnPossess`)
  (`self.K2_DestroyActor` _output_get)
  (`self.Respawn Server` (struct) false))

(event `Return From Firing Range`
  (bind _returnvalue (`GameplayStatics.GetPlayerController` 0))
  (bind _outactors (`GameplayStatics.GetAllActorsOfClass` "/Script/Engine.PlayerStart"))
  (bind _returnvalue_2 (`|SpawnActorFromClass` "/Game/BP/Player/PlayerLobby_BP.PlayerLobby_BP_C" (`self.GetTransform` (`|GetArrayItem` _outactors)) "AlwaysSpawn" "OverrideRootScale" null true null))
  (`self.Possess` _returnvalue_2)
  (bind _returnvalue_3 (`/Game/BP/Main_GI.ChangeWidget` (cast `/Game/BP/Main_GI` (`GameplayStatics.GetGameInstance`) :!pure true) "/Game/BP/UI/MainMenu/Loadout/Loadout_BP.Loadout_BP_C"))
  (set `PlayerController.bShowMouseCursor` true _returnvalue)
  (`WidgetBlueprintLibrary.SetInputMode_UIOnlyEx` _returnvalue null)
  (bind _asloadout_bp (cast `/Game/BP/UI/MainMenu/Loadout/Loadout_BP` _returnvalue_3))
  (set `/Game/BP/UI/MainMenu/Loadout/Loadout_BP.bMainMenu` true _asloadout_bp))

(fn `UserConstructionScript`)