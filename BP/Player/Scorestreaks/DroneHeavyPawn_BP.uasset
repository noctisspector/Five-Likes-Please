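; Heavy drone scorestreak pawn that extends a parent drone with a charged, explosive secondary weapon on the Aim input.
; Pressing Aim calls a server-named event that plays a charge sound and starts a one-shot timer; releasing early cancels it.
; When the timer completes and the drone is alive, it spawns an arcing explosive projectile from FP1, plus a firing sound and attached muzzle flash.
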(event `InputAction|Aim`
  (params (Key :type "Key Structure"))
  ;[1 1 1] Secondary Input
  (:`Pressed`
    (`self.Pressing SECONDARY Server` true))
  (:`Released`
    (`self.Pressing SECONDARY Server` false)))

(event `Pressing SECONDARY Server`
  (params (` ` :type Boolean))
  ;[1 1 1] Secondary Input
  (if ` `
    (`self.SHOOT SECONDARY ON`)
    (else
      (`self.SHOOT SECONDARY OFF`))))

(event `SHOOT SECONDARY OFF`
  ;[1 1 1] Shoot Secondary
  (`KismetSystemLibrary.K2_ClearAndInvalidateTimerHandle` (stale `SHOOT SECONDARY ON` _returnvalue)))

(event `SHOOT SECONDARY ON`
  ;[1 1 1] Shoot Secondary
  (`self.CHARGING Secondary CLient`)
  (bind _returnvalue (`KismetSystemLibrary.K2_SetTimerDelegate` (delegate `Fire SECONDARY Event`) (`self.SECONDARY Fire Delay`))))

(event `Secondary Client`
  (bind _poseablemesh (`self.PoseableMesh`))
  (bind (_returnvalue_location _returnvalue_rotation _returnvalue_scale) (`KismetMathLibrary.BreakTransform` (`SceneComponent.K2_GetComponentToWorld` _poseablemesh)))
  ;[1 1 1] Secondary Client Actions
  (`GameplayStatics.PlaySoundAtLocation` "/Game/ExplosionSoundPack/ProSoundCollectionBonusSoundsMONO/Wavs/sci-fi_weapon_rifle_large_shot_03.sci-fi_weapon_rifle_large_shot_03" (`self.K2_GetActorLocation`) (struct) 1.0 1.0 0.0 "/Game/Sound/Gun_ATT.Gun_ATT" "/Game/Sound/Gun_CON.Gun_CON" self)
  (bind _returnvalue (`|SpawnActorFromClass` (`self.MF Class`) (`KismetMathLibrary.MakeTransform` (`KismetMathLibrary.InverseTransformLocation` (`KismetMathLibrary.MakeTransform` _returnvalue_location _returnvalue_rotation _returnvalue_scale) (`SceneComponent.GetSocketLocation` _poseablemesh "MF1")) (`KismetMathLibrary.MakeRotator` (`KismetMathLibrary.RandomFloatInRange` 0.0 360.0))) "Undefined" "OverrideRootScale" null null))
  (`self.K2_AttachToActor` _returnvalue self "None" "KeepRelative" "KeepRelative" "KeepRelative" true))

(event `Fire SECONDARY Multicast`
  (bind (_returnvalue_location _returnvalue_rotation) (`KismetMathLibrary.BreakTransform` (`SceneComponent.K2_GetComponentToWorld` (`self.FP1`))))
  ;[1 1 1] Shoot Secondary
  (bind _returnvalue (`|SpawnActorFromClass` (`self.SECONDARY Projectile`) (`KismetMathLibrary.MakeTransform` _returnvalue_location _returnvalue_rotation) "AlwaysSpawn" "OverrideRootScale" null self 50.0 "/Game/BP/Weapons/DamageCurves/DamageCurve_Constant.DamageCurve_Constant" 350.0 0.0 "/Game/Sound/ExplosionSoundPack/ExplosionSoundsMONO/Cues/explosion_small_no_tail_02_Cue.explosion_small_no_tail_02_Cue" "/Game/BP/Weapons/Exp/MissileEXP_BP.MissileEXP_BP_C" 3000.0 1.4 1.0 65.0 0.0 false "NewEnumerator0" null 0.0 false false false false "NewEnumerator3" null))
  (`/Game/BP/Weapons/Projectiles/Projectile_BP.Init` _returnvalue 0.35 0.5))

(event `Fire SECONDARY Event`
  ;[1 1 1] Shoot Secondary
  (if (not (`self.bDead`))
    (`self.Fire SECONDARY Multicast`)
    (`self.Secondary Client`)))

(event `CHARGING Secondary CLient`
  (`GameplayStatics.PlaySoundAtLocation` "/Game/ExplosionSoundPack/ProSoundCollectionBonusSounds/Wavs/sci-fi_weapon_reload_06.sci-fi_weapon_reload_06" (`self.K2_GetActorLocation`) (struct) 1.0 1.0 0.0 "/Game/Sound/Gun_ATT.Gun_ATT" "/Game/Sound/Gun_CON.Gun_CON" self))

(fn `UserConstructionScript`
  (`parent.UserConstructionScript`))