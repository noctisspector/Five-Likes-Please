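; Base multiplayer player character that handles health, death, the in-game HUD, chat and scoreboard, with empty hooks for child weapon and ragdoll logic.
; ModifyHealth drives health bars, hurt direction, status effects and server-side death with kill credit, Jug handoff and respawn.
; Tick runs authority regen, minimap updates and line traces that reveal nametags for teammates or the aimed-at player.
; Scoreboard data reaches the HUD through a RepNotify.
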(event `/Game/BP/Player/Player_Interface.END GAME`
  (params (Winner :type String))
  ;[1 1 1] End Game
  (`self.End Game Client` Winner)
  (`self.End Game Local` Winner))

(event `End Game Client`
  (params (Winner :type String))
  ;[1 1 1] End Game
  (`self.End Game Local` Winner))

(event `InputAction|Scoreboard`
  (params (Key :type "Key Structure"))
  (bind _hud (`self.HUD`))
  ;[1 1 1] Scoreboard Show/Hide
  (:`Pressed`
    (`/Game/BP/UI/Ingame/InGameHUD_BP.Show Scoreboard` _hud))
  (:`Released`
    (`/Game/BP/UI/Ingame/InGameHUD_BP.Hide Scoreboard` _hud)))

(event `Update Minimap Rep`
  (bind (_returnvalue_location _returnvalue_rotation) (`KismetMathLibrary.BreakTransform` (`self.GetTransform`)))
  (bind _hud (`self.HUD`))
  ;[1 1 1] Update Minimap Rep
  (`/Engine/EditorBlueprintResources/StandardMacros.IsValid` _hud
    (:`Is Valid`
      (`/Game/BP/UI/Ingame/InGameHUD_BP.Update Minimap Rep` _hud _returnvalue_location _returnvalue_rotation))))

(event `End Game Local`
  (params (Winner :type String))
  (bind _hud (`self.HUD`))
  ;[1 1 1] End Game
  (`/Engine/EditorBlueprintResources/StandardMacros.IsValid` _hud
    (:`Is Valid`
      (`/Engine/EditorBlueprintResources/StandardMacros.DoOnce` false
        (:`Completed`
          (`Widget.RemoveFromParent` _hud))))))

(event `Meme Music Server`
  (`self.Start Meme Music`))

(event `self.ReceiveTick`
  (params (DeltaSeconds :type "Float (single-precision)"))
  (bind _camera (`self.Camera F`))
  (bind (_returnvalue_x _returnvalue_y) (`KismetMathLibrary.BreakVector` (`self.GetActorForwardVector`)))
  (bind _lasthurtdirtarget (`self.LastHurtDirTarget`))
  (bind _hud (`self.HUD`))
  (bind _returnvalue (`SceneComponent.K2_GetComponentLocation` _camera))
  (`|ExecutionSequence`
    (:`then_0`
      ;[1 1 1] Find Looking At Player
      (`self.Multiplayer State`
        (:`Player`
          (bind (_outhit _returnvalue_2) (`KismetSystemLibrary.LineTraceSingle` :`Start` _returnvalue :`End` (+ _returnvalue (`KismetMathLibrary.GreaterGreater_VectorRotator` (200000.0 0.0 0.0) (`SceneComponent.K2_GetComponentRotation` _camera))) :`TraceChannel` "TraceTypeQuery4" :`bTraceComplex` true :`TraceColor` (struct :`R` 1.0 :`B` 0.053742 :`A` 1.0) :`DrawTime` 0.3))
          (if _returnvalue_2
            (bind (_bblockinghit _binitialoverlap _time _distance _location _impactpoint _normal _impactnormal _physmat _hitactor) (`GameplayStatics.BreakHitResult` _outhit))
            (bind (_outhit_2 _returnvalue_3) (`KismetSystemLibrary.LineTraceSingle` _returnvalue (`self.K2_GetActorLocation` _hitactor) "TraceTypeQuery1" true (`|MakeArray` _hitactor)))
            (bind __ (`self.GetRevealDist`))
            (if (and (not _returnvalue_3) (== (`GameplayStatics.GetObjectClass` _hitactor) "/Game/BP/Player/Player_BP.Player_BP_C") (< (`self.GetDistanceTo` _hitactor) __))
              (bind _output_get (set `self.Traced Player` (cast `/BP/Player/PlayerParent_BP` _hitactor :!pure true)))
              (set `self.bTracedSuccess` (not (`/BP/Player/PlayerParent_BP.bDead` _output_get)))
              (else
                (set `self.bTracedSuccess` false :!label _label)))
            (else
              (goto _label)))
          ;[1 1 1] Change Nametag Visibility
          (bind _outactors (`GameplayStatics.GetAllActorsOfClass` "PlayerParent_BP_C"))
          (for _array_element _outactors
            (bind ___2 (`self.(P) Check Team` _array_element))
            (if ___2
              (`self.Set Traced State` _array_element true)
              (elif (and (== _array_element (`self.Traced Player`)) (`self.bTracedSuccess`))
                (`self.Set Traced State` _array_element true)
                (else
                  (`self.Set Traced State` _array_element false))))))))
    (:`then_1`
      ;[1 1 1] HUD Hurt
      (`/Engine/EditorBlueprintResources/StandardMacros.IsValid` _hud
        (:`Is Valid`
          (`/Game/BP/UI/Ingame/InGameHUD_BP.Change Hurt` _hud (`KismetMathLibrary.MapRangeClamped` (- 1.0 (/ (`self.Health`) (`self.(P) Max Health`))) 0.0 1.0 0.0 2.0)))))
    (:`then_2`
      (`self.Update Minimap Rep`))
    (:`then_3`
      (`self.Icon Name & Color`))
    (:`then_4`
      (`self.(P) Regen`))
    (:`then_5`
      ;[1 1 1] Hurt DIR
      (`|ExecutionSequence`
        (:`then_0`
          (`/Engine/EditorBlueprintResources/ActorMacros.Switch Has Authority`
            (:`Authority`
              (`/Engine/EditorBlueprintResources/StandardMacros.IsValid` _lasthurtdirtarget
                (:`Is Valid`
                  (set `self.HurtDirTargetLocation` (`self.K2_GetActorLocation` _lasthurtdirtarget)))))))
        (:`then_1`
          (`/Engine/EditorBlueprintResources/StandardMacros.IsValid` (`self.HUD`)
            (:`Is Valid`
              (bind _output_get_2 (set `self.HurtDirCurrentLocation` (`KismetMathLibrary.VInterpTo` (`self.HurtDirCurrentLocation`) (`self.HurtDirTargetLocation`) (`GameplayStatics.GetWorldDeltaSeconds`) 10.0)))
              (bind (_returnvalue_x_2 _returnvalue_y_2) (`KismetMathLibrary.BreakVector` (- (`self.K2_GetActorLocation`) _output_get_2)))
              (`/Game/BP/UI/Ingame/InGameHUD_BP.UpdateHurtDir` (`self.HUD`) (`KismetMathLibrary.MakeVector2D` _returnvalue_x_2 _returnvalue_y_2) (`KismetMathLibrary.MakeVector2D` _returnvalue_x _returnvalue_y) (`self.K2_GetActorRotation`)))))))))

(event `Key|J`
  (params (Key :type "Key Structure"))
  (:`Pressed`
    (`self.Meme Music Server`)))

(event `Start Meme Music`
  (bind _meme_music (`self.Meme Music`))
  (`/Engine/EditorBlueprintResources/StandardMacros.IsValid` _meme_music
    (:`Is Valid`
      (`ActorComponent.K2_DestroyComponent` _meme_music))
    (:`Is Not Valid`
      _))
  (bind _returnvalue (`GameplayStatics.SpawnSoundAttached` "/Game/Sound/Music/MemeMusic_CUE.MemeMusic_CUE" (`self.CapsuleComponent`) "None" (0.0 0.0 0.0) (struct) "KeepRelativeOffset" true 1.0 1.0 0.0 "/Game/Sound/Meme_ATT.Meme_ATT" null))
  (bind _output_get (set `self.Meme Music` _returnvalue))
  (`ActorComponent.Activate` _output_get false))

(event `Icon Name & Color`
  (bind _asmain_player_state_bp (`self.Player State`))
  (bind _playerstate (`Controller.PlayerState` (`GameplayStatics.GetPlayerController` 0)))
  ;[1 1 1] Set Name Icon & Color
  (`/Engine/EditorBlueprintResources/StandardMacros.IsValid` _playerstate
    (:`Is Valid`
      (`/Engine/EditorBlueprintResources/StandardMacros.IsValid` _asmain_player_state_bp
        (:`Is Valid`
          (`/Game/BP/UI/Ingame/HealthBar_BP.Set Name` (cast `/Game/BP/UI/Ingame/HealthBar_BP` (`WidgetComponent.GetUserWidgetObject` (`self.Health Bar`)) :!pure true) (`/Game/BP/Player/MainPlayerState_BP.Name` _asmain_player_state_bp) (and (`self.(P) Have Teams`) (== (`/Game/BP/Player/MainPlayerState_BP.Team` _asmain_player_state_bp) (`/Game/BP/Player/MainPlayerState_BP.Team` (cast `/Game/BP/Player/MainPlayerState_BP` _playerstate :!pure true))))))))))

(event `self.ReceiveBeginPlay`
  (`|ExecutionSequence`
    (:`then_0`
      (`/Engine/EditorBlueprintResources/ActorMacros.Switch Has Authority`
        (:`Authority`
          (set `self.Health Mod` (`/Game/BP/Main_GI.Health Mod` (`self.GI`))))))
    (:`then_1`
      (`self.Multiplayer State`
        (:`Player`
          (`PrimitiveComponent.SetRenderCustomDepth` (`self.Mesh`) false))))))

(event `Update Healthbar Multicast P`
  (params (bNoFlinch :type Boolean) (`Shot Delay` :type "Float (double-precision)"))
  (`self.(P) Update Local Health Bar`))

(event `Suicide`
  (`self.ModifyHealth` -999999.0 self (0.0 0.0 0.0) false false "NewEnumerator0" false false 1.0))

(event `Kill HUD`
  (params (Score :type "Float (double-precision)") (Likes :type Integer))
  (bind _hud (`self.HUD`))
  ;[1 1 1] Kill HUD
  (`/Engine/EditorBlueprintResources/StandardMacros.IsValid` _hud
    (:`Is Valid`
      (`/Game/BP/UI/Ingame/InGameHUD_BP.Visual Score` _hud Score Likes))))

(event `Objective Score`
  ;[1 1 1] Kill Score
  (`/Engine/EditorBlueprintResources/ActorMacros.Switch Has Authority`
    (:`Authority`
      (bind _asmp_point_gm (cast `/Game/BP/GameModes/MP_POINT_GM` (`GameplayStatics.GetGameMode`) :!label _label))
      (`self.Kill HUD` (`/Game/BP/GameModes/MP_Base_GM.Objective Capture Score` _asmp_point_gm)))
    (:`Remote`
      (`self.Objective Score Server`))))

(event `Objective Score Server`
  ;[1 1 1] Kill Score
  (goto _label))

(event `Killed Enemy`
  ;[1 1 1] Kill Score
  (`/Engine/EditorBlueprintResources/ActorMacros.Switch Has Authority`
    (:`Authority`
      (bind _asmp_base_gm (cast `/Game/BP/GameModes/MP_Base_GM` (`GameplayStatics.GetGameMode`) :!label _label_2))
      (`/Game/BP/GameModes/MP_Base_GM.Player Kill` _asmp_base_gm self)
      (`self.Kill HUD` (`/Game/BP/GameModes/MP_Base_GM.Kill Score` _asmp_base_gm) (`/Game/BP/GameModes/MP_Base_GM.Kill Likes` _asmp_base_gm))
      (`self.Trigger Next Weapon (OVERRIDE)`)
      (`KismetSystemLibrary.PrintString` "Hello"))
    (:`Remote`
      (`self.Killed Enemy Server`))))

(event `Killed Enemy Server`
  ;[1 1 1] Kill Score
  (goto _label_2))

(event `ModifyHealth`
  (params (Amount :type "Float (double-precision)") (Instigator :type "/BP/Player/PlayerParent_BP Object Reference") (Force :type "Vector Structure") (bForce :type Boolean) (bNoRegenReset :type Boolean) (StatusEffect :type "/Game/BP/Weapons/Equiptment/StatusEffect Enum" :default "NewEnumerator0") (bNoJug :type Boolean) (bHeadshot :type Boolean) (ShotDelay :type "Float (double-precision)"))
  (bind _returnvalue (`self.(P) Max Health`))
  (bind _name (`/Game/BP/Player/MainPlayerState_BP.Name` (cast `/Game/BP/Player/MainPlayerState_BP` (`Pawn.PlayerState` Instigator) :!pure true)))
  (set `self.LastHurtDirTarget` Instigator)
  (`|ExecutionSequence`
    (:`then_0`
      (if bForce
        (set `self.Last Force` Force))
      (bind _output_get (set `self.Health` (`KismetMathLibrary.FClamp` (+ (`self.Health`) Amount) 0.0 _returnvalue)))
      (if (not bNoRegenReset)
        (set `self.Health Regen Counter` 0.0))
      (`self.Update Health Bar (OVERRIDE)` (/ _output_get _returnvalue))
      (`|ExecutionSequence`
        (:`then_0`
          (if (<= (`self.Health`) 0.0)
            (`/Engine/EditorBlueprintResources/ActorMacros.Switch Has Authority`
              (:`Authority`
                (`/Engine/EditorBlueprintResources/StandardMacros.DoOnce` false
                  (:`Completed`
                    (`self.Kill Server` bNoJug)
                    (`/Engine/EditorBlueprintResources/StandardMacros.IsValid` Instigator
                      (:`Is Valid`
                        (`self.Killed Enemy` Instigator)
                        (`self.Hitmarker` Instigator true bHeadshot (`self.Player Name`))
                        ;[1 1 1] Chat Death
                        (`self.AddChat_Server` (select `bool` (not (`KismetStringLibrary.EqualEqual_StrStr` _name)) :`false` (`|MakeArray` (make `/Game/BP/UI/ChatContent` (`KismetTextLibrary.Conv_StringToText` (`self.Player Name`)) (make `SlateColor` (struct :`R` 0.419608 :`G` 0.419608 :`B` 0.419608 :`A` 1.0))) (make `/Game/BP/UI/ChatContent` (`KismetTextLibrary.Conv_StringToText` " was hit by a Russian shell") (make `SlateColor` (struct :`R` 1.0 :`G` 0.090196 :`B` 0.090196 :`A` 1.0))) :!type "/Game/BP/UI/ChatContent Structure") :`true` (`|MakeArray` (make `/Game/BP/UI/ChatContent` (`KismetTextLibrary.Conv_StringToText` _name) (make `SlateColor` (struct :`R` 0.419608 :`G` 0.419608 :`B` 0.419608 :`A` 1.0))) (make `/Game/BP/UI/ChatContent` (`KismetTextLibrary.Conv_StringToText` " killed ") (make `SlateColor` (struct :`R` 1.0 :`G` 0.090196 :`B` 0.090196 :`A` 1.0))) (make `/Game/BP/UI/ChatContent` (`KismetTextLibrary.Conv_StringToText` (`self.Player Name`)) (make `SlateColor` (struct :`R` 0.489583 :`G` 0.489583 :`B` 0.489583 :`A` 1.0))) :!type "/Game/BP/UI/ChatContent Structure")))))))))))
        (:`then_1`
          (`self.Update Health Bar Multicast (OVERRIDE)` bNoRegenReset ShotDelay))))
    (:`then_1`
      (`self.StatusEffectClient` StatusEffect Instigator bNoRegenReset))))

(event `Remove HUD Multicast`
  (bind _hud (`self.HUD`))
  (bind _pause_hud (`self.Pause HUD`))
  (`/Engine/EditorBlueprintResources/StandardMacros.IsValid` _hud
    (:`Is Valid`
      (`Widget.RemoveFromParent` _hud)
      (`Widget.SetVisibility` _hud "Hidden"))
    (:`Is Not Valid`
      _))
  (`/Engine/EditorBlueprintResources/StandardMacros.IsValid` _pause_hud
    (:`Is Valid`
      (`Widget.RemoveFromParent` _pause_hud)
      (`Widget.SetVisibility` _pause_hud "Hidden"))))

(event `Kill Server`
  (params (NoJug :type Boolean))
  (bind _asmain_player_state_bp (`self.Player State`))
  (`|ExecutionSequence`
    (:`then_0`
      ;[1 1 1] Next Jug
      (if NoJug
        _
        (elif (`/Game/BP/Player/MainPlayerState_BP.bJug` _asmain_player_state_bp)
          (`/Game/BP/Player/MainPlayerState_BP.Next Jug` _asmain_player_state_bp))))
    (:`then_1`
      (set `self.bDead` true)
      (`self.Destroy Weapon (OVERRIDE)`)
      (`self.Remove HUD Multicast`)
      (`self.Ragdoll (OVERRIDE)`)
      (`self.Hide Mesh Multicast`)
      (bind _asplayer_controller_game_bp (cast `/Game/BP/Player/PlayerControllerGame_BP` (`self.GetController`)))
      (`/Game/BP/Player/PlayerControllerGame_BP.Respawn Server` _asplayer_controller_game_bp (`self.GetTransform`) true (stale `ModifyHealth` Instigator))
      (`KismetSystemLibrary.Delay` (`self.Kill Timer`))
      (`self.K2_DestroyActor`))))

(event `Hide Mesh Multicast`
  (`SceneComponent.SetVisibility` (`self.Mesh`) (not (`self.bHideMeshOnDeath`)) false))

(event `StatusEffectClient`
  (params (Effect :type "/Game/BP/Weapons/Equiptment/StatusEffect Enum" :default "NewEnumerator0") (Inst :type "/BP/Player/PlayerParent_BP Object Reference") (noRegenReset :type Boolean))
  ;[1 1 1] Status Effects
  (`self.StatusEffectLocal` Effect Inst noRegenReset))

(event `StatusEffectLocal`
  (params (Effect :type "/Game/BP/Weapons/Equiptment/StatusEffect Enum" :default "NewEnumerator0") (Inst :type "/BP/Player/PlayerParent_BP Object Reference") (noRegenReset :type Boolean))
  (bind _returnvalue (`self.K2_GetActorLocation`))
  (bind _stuneffects (`self.StunEffects`))
  (bind _hud (`self.HUD`))
  (bind _stuneffects_2 (`self.StunEffects`))
  (bind _hud_2 (`self.HUD`))
  ;[1 1 1] Status Effects
  (`/Engine/EditorBlueprintResources/StandardMacros.IsValid` _hud_2
    (:`Is Valid`
      (if (not noRegenReset)
        (set `self.HurtDirCurrentLocation` (`self.HurtDirTargetLocation`))
        (`/Game/BP/UI/Ingame/InGameHUD_BP.TriggerHurtDir` _hud_2)))
    (:`Is Not Valid`
      _))
  (switch `/Game/BP/Weapons/Equiptment/StatusEffect` Effect
    (:`NewEnumerator1`
      (`/Engine/EditorBlueprintResources/StandardMacros.IsValid` _hud
        (:`Is Valid`
          (`/Game/BP/UI/Ingame/InGameHUD_BP.Flash` _hud 1.0))))
    (:`NewEnumerator2`
      (`/Engine/EditorBlueprintResources/StandardMacros.IsValid` _hud
        (:`Is Valid`
          (`/Game/BP/UI/Ingame/InGameHUD_BP.Stun` _hud 1.0)
          (bind (_direction _value _post) (`Timeline|Timeline_0` :!via `PlayFromStart` :!label _label)
            (:`Update`
              (set `self.Stun Mod` _value)
              (`self.Multiplayer State`
                (:`Player`
                  (set `PostProcessComponent.BlendWeight` _post _stuneffects))))
            (:`Finished`
              (set `self.Stun Mod` 1.0)
              (`self.Multiplayer State`
                (:`Player`
                  (set `PostProcessComponent.BlendWeight` _post _stuneffects))))))
        (:`Is Not Valid`
          (goto _label :!via `PlayFromStart`))))
    (:`NewEnumerator3`
      (`/Engine/EditorBlueprintResources/StandardMacros.IsValid` _hud
        (:`Is Valid`
          (`/Game/BP/UI/Ingame/InGameHUD_BP.Stun` _hud 2.5)
          (bind (_direction_2 _value_2 _post_2) (`Timeline|Timeline_1` :!via `PlayFromStart` :!label _label_2)
            (:`Update`
              (set `self.Stun Mod` _value_2)
              (`self.Multiplayer State`
                (:`Player`
                  (set `PostProcessComponent.BlendWeight` _post_2 _stuneffects_2))))
            (:`Finished`
              (set `self.Stun Mod` 1.0)
              (`self.Multiplayer State`
                (:`Player`
                  (set `PostProcessComponent.BlendWeight` _post_2 _stuneffects_2))))))
        (:`Is Not Valid`
          (goto _label_2 :!via `PlayFromStart`))))
    (:`NewEnumerator4`
      (`/Engine/EditorBlueprintResources/StandardMacros.IsValid` _hud
        (:`Is Valid`
          (`/Game/BP/UI/Ingame/InGameHUD_BP.Flash` _hud 5.0))))
    (:`NewEnumerator6`
      ;[1 1 1] Shocking
      (bind _outactors (`GameplayStatics.GetAllActorsOfClass` "PlayerParent_BP_C"))
      (for _array_element _outactors
        (if (< (`self.GetDistanceTo` _array_element self) (`self.Shock Distance`))
          (`|ExecutionSequence`
            (:`then_0`
              (`/Engine/EditorBlueprintResources/ActorMacros.Switch Has Authority`
                (:`Authority`
                  (if (!= _array_element Inst)
                    (`self.ModifyHealth` _array_element (`self.Shock Damage`) Inst (0.0 0.0 0.0) true false "NewEnumerator4" false false 0.1)))))
            (:`then_1`
              (bind _returnvalue_2 (`self.K2_GetActorLocation` _array_element))
              (if (not (== _returnvalue _returnvalue_2 :`ErrorTolerance` 2.0))
                (`/Game/BP/Main_GI.Spawn Tracer` (`self.GI`) "/Game/FX/Tracer/ShockTracer_P.ShockTracer_P" _returnvalue _returnvalue_2)))))))))

(event `Hitmarker`
  (params (Kill :type Boolean) (Headshot :type Boolean) (Name :type String))
  (bind _hud (`self.HUD`))
  ;[1 1 1] Hitmarker
  (`/Engine/EditorBlueprintResources/StandardMacros.IsValid` _hud
    (:`Is Valid`
      (`/Game/BP/UI/Ingame/InGameHUD_BP.Hitmarker` _hud Kill Headshot Name)
      (if Kill
        (`GameplayStatics.PlaySound2D` "/Game/Sound/RAW/HitmarkerDeath_Cue.HitmarkerDeath_Cue" 2.0 1.0 0.0 "/Game/Sound/Hit_Con.Hit_Con" null)
        (else
          (`GameplayStatics.PlaySound2D` "/Game/Sound/RAW/Hitmarker_Cue.Hitmarker_Cue" 0.5 1.0 0.0 "/Game/Sound/Hit_Con.Hit_Con" null))))))

(event `BlastToShadowRealm`
  (`self.ModifyHealth` -999999.0 self (-100000000.0 0.0 0.0) true false "NewEnumerator0" false false 1.0))

(event `InputAction|Interact`
  (params (Key :type "Key Structure"))
  ;[1 1 1] Interaction
  (:`Pressed`
    (if (`self.bOnLever`)
      (`self.Interact Server`))))

(event `Interact Server`
  ;[1 1 1] Interaction
  (bind _outactors (`GameplayStatics.GetAllActorsOfClass` "/Game/BP/Environment/EventDoorLever_BP.EventDoorLever_BP_C"))
  (for _array_element _outactors
    (`/Game/BP/Environment/EventDoorLever_BP.ToggleLever` _array_element)))

(event `Keytip`
  (params (`Key Message` :type String) (InActionName :type Name))
  (bind _hud (`self.HUD`))
  ;[1 1 1] Keytip
  (`/Engine/EditorBlueprintResources/StandardMacros.IsValid` _hud
    (:`Is Valid`
      (`/Game/BP/UI/Ingame/InGameHUD_BP.Start Keytip` _hud (`.Key` (break `InputActionKeyMapping` (`|GetArrayItem` (`InputSettings.GetActionMappingByName` (`InputSettings.GetInputSettings`) InActionName)))) `Key Message`))))

(event `Key|AnyKey`
  (params (Key :type "Key Structure"))
  ;[1 1 1] Any Key Input
  (:`Pressed`
    (set `/Game/BP/Main_GI.LastKey` Key (`self.GI`))))

(event `InputAction|Spectate`
  (params (Key :type "Key Structure"))
  ;[1 1 1] Spectate'
  (:`Released`
    (`Widget.RemoveFromParent` (`self.HUD`))
    (bind _asplayer_controller_game_bp (cast `/Game/BP/Player/PlayerControllerGame_BP` (`self.GetController`)))
    (`/Game/BP/Player/PlayerControllerGame_BP.Begin Spectate` _asplayer_controller_game_bp)))

(event `InputAction|Chat`
  (params (Key :type "Key Structure"))
  (bind _hud (`self.HUD`))
  ;[1 1 1] Chat Input
  (:`Pressed`
    (bind _asplayer_controller (cast `PlayerController` (`self.GetController`)))
    (`WidgetBlueprintLibrary.SetInputMode_UIOnlyEx` _asplayer_controller _hud)
    (`/Game/BP/UI/Ingame/InGameHUD_BP.TryChat` _hud self)))

(event `AddChat_Server`
  (params (Content :type "Array of /Game/BP/UI/ChatContent Structure (by ref)"))
  ;[1 1 1] Add Chat
  (bind _outactors (`GameplayStatics.GetAllActorsOfClass` "PlayerParent_BP_C"))
  (for _array_element _outactors
    (`self.AddChat_Multi` _array_element Content)))

(event `AddChat_Multi`
  (params (Content :type "Array of /Game/BP/UI/ChatContent Structure (by ref)"))
  (bind _hud (`self.HUD`))
  ;[1 1 1] Add Chat
  (`/Engine/EditorBlueprintResources/StandardMacros.IsValid` _hud
    (:`Is Valid`
      (`/Game/BP/UI/Ingame/InGameHUD_BP.AddChat` _hud Content))))

(event `Finished Chat`
  (params (Message :type Text))
  ;[1 1 1] Chat Input
  (bind _asplayer_controller (cast `PlayerController` (`self.GetController`)))
  (`WidgetBlueprintLibrary.SetInputMode_GameOnly` _asplayer_controller)
  (`self.AddChat_Server` (`|MakeArray` (make `/Game/BP/UI/ChatContent` (`KismetTextLibrary.Conv_StringToText` (`self.Player Name`)) (make `SlateColor` (struct :`R` 0.969681 :`G` 1.0 :`B` 0.548104 :`A` 1.0))) (make `/Game/BP/UI/ChatContent` (`KismetTextLibrary.Conv_StringToText` " - ") (make `SlateColor` (struct :`R` 1.0 :`G` 1.0 :`B` 1.0 :`A` 1.0))) (make `/Game/BP/UI/ChatContent` Message (make `SlateColor` (struct :`R` 1.0 :`G` 1.0 :`B` 1.0 :`A` 1.0))) :!type "/Game/BP/UI/ChatContent Structure")))

(fn `(P) Check Team`
  (params (Other :type "Pawn Object Reference"))
  (returns (` ` :type Boolean))
  (bind _asmain_player_state_bp (`self.Player State`))
  (bind _playerstate (`Pawn.PlayerState` Other))
  (if (`KismetSystemLibrary.IsValid` _playerstate)
    (return (and (`self.(P) Have Teams`) (select `bool` (and (`KismetSystemLibrary.IsValid` _asmain_player_state_bp) (`KismetSystemLibrary.IsValid` _playerstate)) :`true` (== (`/Game/BP/Player/MainPlayerState_BP.Team` _asmain_player_state_bp) (`/Game/BP/Player/MainPlayerState_BP.Team` (cast `/Game/BP/Player/MainPlayerState_BP` _playerstate :!pure true))))))
    (else
      (return false))))

(fn `(P) Have Teams`
  (returns (` ` :type Boolean))
  (return (or (`|EnumEquality` (`self.Win Condition`) "NewEnumerator1") (== (`GameplayStatics.GetObjectClass` (`GameplayStatics.GetGameMode`)) "/Game/BP/GameModes/MP_JUG_GM.MP_JUG_GM_C"))))

(fn `(P) Init Health`
  (set `self.Health` (`self.(P) Max Health`)))

(fn `(P) Init HUD`
  (`self.Multiplayer State`
    (:`Player`
      (`/Engine/EditorBlueprintResources/StandardMacros.DoOnce` false
        (:`Completed`
          (`/Engine/EditorBlueprintResources/StandardMacros.IsValid` (`self.HUD`)
            (:`Is Not Valid`
              (bind _returnvalue (`|CreateWidget` "/Game/BP/UI/Ingame/InGameHUD_BP.InGameHUD_BP_C" (`GameplayStatics.GetPlayerController` 0)))
              (bind _output_get (set `self.HUD` _returnvalue))
              (`UserWidget.AddToViewport` _output_get 0)
              (if (`self.bOverrideReticule`)
                (`/Game/BP/UI/Ingame/InGameHUD_BP.CustomReticule` _output_get (`self.CustomReticule`))))))))))

(fn `(P) Max Health`
  (returns (ReturnValue :type "Float (double-precision)"))
  (bind _asmain_player_state_bp (`self.Player State`))
  (bind _max_health (`self.Max Health`))
  (bind _health_mod_modifier (break `/Game/BP/GameModes/HealthModProperties` (`self.Health Mod`)))
  (return (* (select `bool` (select `bool` (`KismetSystemLibrary.IsValid` _asmain_player_state_bp) :`true` (`/Game/BP/Player/MainPlayerState_BP.bJug` _asmain_player_state_bp)) :`false` _max_health :`true` (* _max_health (`self.JUG Health Mp`))) _health_mod_modifier)))

(fn `(P) Regen`
  (bind _returnvalue (`GameplayStatics.GetWorldDeltaSeconds`))
  (bind _asmain_player_state_bp (`self.Player State`))
  ;[1 1 1] Regen
  (`/Engine/EditorBlueprintResources/ActorMacros.Switch Has Authority`
    (:`Authority`
      (`/Engine/EditorBlueprintResources/StandardMacros.IsValid` _asmain_player_state_bp
        (:`Is Valid`
          (set `self.Health Regen Counter` (+ (`self.Health Regen Counter`) _returnvalue))
          (if (and (> (`self.Health Regen Counter`) (`self.Health Regen Delay`)) (< (`self.Health`) (`self.(P) Max Health`)) (not (`/Game/BP/Player/MainPlayerState_BP.bJug` _asmain_player_state_bp)))
            (`self.ModifyHealth` (* (`self.Health Regen`) _returnvalue) null (0.0 0.0 0.0) false true)))))))

(fn `(P) Update Local Health Bar`
  (`self.Multiplayer State`
    (:`Player`
      (`/Game/BP/UI/Ingame/InGameHUD_BP.Update Health` (`self.HUD`) (/ (`self.Health`) 1.0)))))

(fn `(P) Update Scoreboard`
  (params (`Player States` :type "Array of /Game/BP/Player/MainPlayerState_BP Object Reference") (`Win Condition` :type "/Game/BP/GameModes/WinCondition Enum" :default "NewEnumerator0") (`Team Score` :type "Array of Float (double-precision)") (Time :type "Float (double-precision)") (`End Condition` :type "/Game/BP/GameModes/EndCondition Enum" :default "NewEnumerator0"))
  (locals (`Player Output` :type "Array of /Game/BP/Player/ScoreInfoPlayer Structure"))
  (bind _asmain_player_state_bp (`self.Player State`))
  (set `self.Local Player States` `Player States`)
  (set `self.Win Condition` `Win Condition`)
  (`/Engine/EditorBlueprintResources/ActorMacros.Switch Has Authority`
    (:`Authority`
      (for _array_element (`self.Local Player States`)
        (`KismetArrayLibrary.Array_Add` (`local.Player Output`) (make `/Game/BP/Player/ScoreInfoPlayer` (`/Game/BP/Player/MainPlayerState_BP.Name` _array_element) (`/Game/BP/Player/MainPlayerState_BP.Local Score` _array_element) (`PlayerState.Ping` _array_element) (`/Game/BP/Player/MainPlayerState_BP.Team` _array_element) (`/Game/BP/Player/MainPlayerState_BP.Local Likes` _array_element))))
      (set `self.Local Player Score` (`/Game/BP/Player/MainPlayerState_BP.Local Score` _asmain_player_state_bp))
      (set `self.Local Player Likes` (`/Game/BP/Player/MainPlayerState_BP.Local Likes` _asmain_player_state_bp))
      (set `self.Scoreboard Data` (make `/Game/BP/Player/ScoreInfo` (`local.Player Output`) `Win Condition` `Team Score` Time `End Condition`)))))

(fn `Camera F`
  (returns (Camera :type "CameraComponent Object Reference"))
  (return null))

(fn `Destroy Weapon (OVERRIDE)`)

(fn `GetRevealDist`
  (returns (` ` :type "Float (double-precision)"))
  (return 900000.0))

(fn `OnRep_Scoreboard Data`
  (bind _hud (`self.HUD`))
  (`/Engine/EditorBlueprintResources/StandardMacros.IsValid` _hud
    (:`Is Valid`
      (`/Game/BP/UI/Ingame/InGameHUD_BP.Populate Scoreboard` _hud (`self.Scoreboard Data`))
      (`/Game/BP/UI/Ingame/InGameHUD_BP.Update Total Score` _hud (`self.Local Player Score`) (`self.Local Player Likes`)))))

(fn `Ragdoll (OVERRIDE)`)

(fn `Set Traced State`
  (params (bVisibleNametag :type Boolean))
  (`SceneComponent.SetVisibility` (`self.Health Bar`) bVisibleNametag false))

(fn `Trigger Next Weapon (OVERRIDE)`)

(fn `Update Health Bar (OVERRIDE)`
  (params (` ` :type "Float (double-precision)"))
  (`/Game/BP/UI/Ingame/HealthBar_BP.Update Health` (cast `/Game/BP/UI/Ingame/HealthBar_BP` (`WidgetComponent.GetUserWidgetObject` (`self.Health Bar`)) :!pure true) ` `))

(fn `Update Health Bar Multicast (OVERRIDE)`
  (params (NoFlicnh :type Boolean) (ShotDelay :type "Float (double-precision)" :default 1.0))
  (`self.Update Healthbar Multicast P` NoFlicnh ShotDelay))

(fn `UserConstructionScript`)