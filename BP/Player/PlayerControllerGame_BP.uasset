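; Player controller for multiplayer matches, handling spawning, respawning, killcam, spectating, pause/quit, the end-game screen and Gun Game weapon progression.
; Deaths route through RespawnServer, optionally possessing a timed replay camera, then show the respawn menu, or respawn immediately in the lobby.
; SpawnServer possesses the chosen player type at the spawn point with the greatest summed distance from opponents.
; NextWeapon advances the game mode's gun list, declaring a win at its end.
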(event `GetPlayers`
  (set `self.GetPlayersString` "")
  (bind _outactors (`GameplayStatics.GetAllActorsOfClass` "PlayerControllerGame_BP_C"))
  (for _array_element _outactors
    (set `self.GetPlayersString` (`KismetStringLibrary.Concat_StrStr` (`self.GetPlayersString`) (`KismetSystemLibrary.GetDisplayName` _array_element) ", ")))
  (`KismetSystemLibrary.PrintString` (`self.GetPlayersString`) true true (struct :`R` 1.0 :`G` 0.01394 :`A` 1.0) 99999.0))

(event `Pending WinScreen`
  (params (Winner :type String))
  ;[1 1 1] Pending Win
  (set `self.bWin` true)
  (bind _returnvalue (`|CreateWidget` "/Game/BP/UI/Ingame/EndGameScreen_BP.EndGameScreen_BP_C" self))
  (bind _output_get (set `self.End Screen` _returnvalue))
  (`UserWidget.AddToViewport` _output_get 0)
  (`WidgetBlueprintLibrary.SetInputMode_UIOnlyEx` self _output_get)
  (set `self.bShowMouseCursor` true)
  (`/Game/BP/UI/Ingame/EndGameScreen_BP.Init` _output_get Winner))

(event `self.ReceiveBeginPlay`
  (if (not (`self.bLobby`))
    (`self.Respawn Server` (struct) false)))

(event `Set Player Type Server`
  (params (`Player Type` :type "/Game/BP/Player/PlayerParent_BP Class Reference"))
  ;[1 1 1] Player Type
  (set `self.Player Type` `Player Type`))

(event `Spawn Server`
  ;[1 1 1] Spawn
  (`self.Spawn Client`)
  (bind _outactors (`GameplayStatics.GetAllActorsOfClass` "/Game/BP/Game/SpawnPoint_BP.SpawnPoint_BP_C"))
  (bind _outactors_2 (`GameplayStatics.GetAllActorsOfClass` "/Game/BP/Player/PlayerParent_BP.PlayerParent_BP_C"))
  (bind _______ (`self.Find Spawn` _outactors _outactors_2 (`/Game/BP/Player/MainPlayerState_BP.Team` (cast `/Game/BP/Player/MainPlayerState_BP` (`self.PlayerState`) :!pure true))))
  (bind _returnvalue (`|SpawnActorFromClass` (`self.Player Type`) (`self.GetTransform` _______) "AlwaysSpawn" "OverrideRootScale" null (`self.bLobby`) (`.bSuccess` (cast `/Game/BP/GameModes/MP_GG_GM` (`GameplayStatics.GetGameMode`) :!pure true)) null))
  (`self.Possess` _returnvalue)
  (`/Game/BP/Player/Player_Interface.SET UP` _returnvalue))

(event `Init Spawn`
  ;[1 1 1] Player Type
  (`self.Set Player Type Server` (`/Game/BP/Main_GI.Player Type` (cast `/Game/BP/Main_GI` (`GameplayStatics.GetGameInstance`) :!pure true)))
  (`self.Spawn Server`))

(event `Spawn Client`
  ;[1 1 1] Spawn
  (`WidgetBlueprintLibrary.SetInputMode_GameOnly` self)
  (set `self.bShowMouseCursor` false))

(event `Respawn Client`
  (if (`self.bLobby`)
    (`self.Init Spawn`)
    (elif (not (`self.bWin`))
      (bind _returnvalue (`|CreateWidget` "/Game/BP/UI/Ingame/RespawnMenu_BP.RespawnMenu_BP_C" self))
      (bind _output_get (set `self.RespawnMenu` _returnvalue))
      (`UserWidget.AddToViewport` _output_get 0)
      (`WidgetBlueprintLibrary.SetInputMode_GameAndUIEx` self _output_get "DoNotLock" false)
      (set `self.bShowMouseCursor` true))))

(event `Respawn Server`
  (params (KillcamTransform :type "Transform Structure") (bKillcam :type Boolean :default true) (Inst :type "/Game/BP/Player/PlayerParent_BP Object Reference"))
  ;[1 1 1] Kill Cam
  (`self.UnPossess`)
  (if bKillcam
    (bind _returnvalue (`|SpawnActorFromClass` "/Game/BP/Player/ReplayCamera_BP.ReplayCamera_BP_C" KillcamTransform "Undefined" "OverrideRootScale" null Inst null))
    (bind _output_get (set `self.ReplayCamera` _returnvalue))
    (`self.Possess` _output_get)
    (`KismetSystemLibrary.Delay` (`self.Killcam Timer`))
    (`self.UnPossess`)
    (`/Game/BP/Player/ReplayCamera_BP.Kill Replay` _output_get))
  (`self.Respawn Client`))

(event `InputAction|Pause`
  (params (Key :type "Key Structure"))
  (bind _returnvalue (`self.K2_GetPawn`))
  ;[1 1 1] Pause
  (:`Pressed`
    (`/Engine/EditorBlueprintResources/StandardMacros.IsValid` _returnvalue
      (:`Is Valid`
        (bind _asplayer_parent_bp (cast `/Game/BP/Player/PlayerParent_BP` _returnvalue)
          (:`then`
            (if (`/Game/BP/Player/PlayerParent_BP.bFiringRange` _asplayer_parent_bp)
              (bind _asplayer_controller_lobby_bp (cast `/Game/BP/Player/PlayerController_Lobby_BP` self))
              (`/Game/BP/Player/PlayerController_Lobby_BP.Return From Firing Range` _asplayer_controller_lobby_bp)
              (`Widget.RemoveFromParent` (`/Game/BP/Player/PlayerParent_BP.HUD` _asplayer_parent_bp))
              (`self.K2_DestroyActor` _asplayer_parent_bp)
              (else
                (bind _returnvalue_2 (`|CreateWidget` "/Game/BP/UI/Ingame/Pause_BP.Pause_BP_C" self :!label _label))
                (`UserWidget.AddToViewport` _returnvalue_2 999999))))
          (:`CastFailed`
            (goto _label))))
      (:`Is Not Valid`
        (goto _label)))))

(event `Quit Button`
  (params (bIterative :type Boolean))
  (bind _returnvalue (`self.K2_GetPawn`))
  ;[1 1 1] Pause
  (`DestroySessionCallbackProxy.DestroySession` (`GameplayStatics.GetPlayerController` 0)
    (:`then`
      (`GameplayStatics.OpenLevel` "Lobby")
      (`self.Destroy Server`)
      (`/Engine/EditorBlueprintResources/StandardMacros.IsValid` _returnvalue :!label _label_2
        (:`Is Valid`
          (`self.K2_DestroyActor` _returnvalue))))))

(event `Destroy Server`
  ;[1 1 1] Pause
  (`self.Destroy Clients`))

(event `Destroy Clients`
  ;[1 1 1] Pause
  (goto _label_2))

(event `End Spectate`
  (`self.K2_DestroyActor` (`self.K2_GetPawn`))
  (`self.Possess` (`self.Previous Pawn`)))

(event `Begin Spectate`
  (bind _output_get (set `self.Previous Pawn` (`self.K2_GetPawn`)))
  (bind _returnvalue (`|SpawnActorFromClass` "/Game/BP/Player/Spectator_BP.Spectator_BP_C" (`self.GetTransform` _output_get) "AlwaysSpawn" "OverrideRootScale" null null))
  (`self.Possess` _returnvalue))

(fn `Find Spawn`
  (params (Spawns :type "Array of /Game/BP/Game/SpawnPoint_BP Object Reference (by ref)") (Players :type "Array of /Game/BP/Player/PlayerParent_BP Object Reference") (Team :type Integer))
  (returns (`      ` :type "/Game/BP/Game/SpawnPoint_BP Object Reference"))
  (locals (`Selected Point` :type "/Game/BP/Game/SpawnPoint_BP Object Reference") (Locations :type "Array of Vector Structure") (`Global Max` :type "Float (double-precision)") (`Local Max` :type "Float (double-precision)"))
  (set `local.Selected Point` (`|GetArrayItem` Spawns))
  ;[1 1 1] Get Player Locations
  (for _array_element Players
    (bind _playerstate (`Pawn.PlayerState` _array_element))
    (`/Engine/EditorBlueprintResources/StandardMacros.IsValid` _playerstate
      (:`Is Valid`
        (if (or (not (== (`/Game/BP/Player/MainPlayerState_BP.Team` (cast `/Game/BP/Player/MainPlayerState_BP` _playerstate :!pure true)) Team)) (not (`/Game/BP/Player/PlayerParent_BP.(P) Have Teams` _array_element)))
          (`KismetArrayLibrary.Array_Add` (`local.Locations`) (`self.K2_GetActorLocation` _array_element))))))
  ;[1 1 1] Find Best Spawn
  (for _array_element_2 Spawns
    (set `local.Local Max` 0.0)
    (for _array_element_3 (`local.Locations`)
      (set `local.Local Max` (+ (* (`KismetMathLibrary.Vector_Distance` (`self.K2_GetActorLocation` _array_element_2) _array_element_3) 0.001) (`local.Local Max`))))
    (if (> (`local.Local Max`) (`local.Global Max`))
      (set `local.Selected Point` _array_element_2)
      (set `local.Global Max` (`local.Local Max`))))
  (return (`local.Selected Point`)))

(fn `Next Weapon`
  (params (bAfterInit :type Boolean))
  (bind _gungameindex (`self.GunGameIndex`))
  (if bAfterInit
    (`/Engine/EditorBlueprintResources/StandardMacros.IncrementInt` (`self.GunGameIndex`)
      (:`  `
        _)))
  (bind _asmp_gg_gm (cast `/Game/BP/GameModes/MP_GG_GM` (`GameplayStatics.GetGameMode`)))
  (bind _gunlist (`/Game/BP/GameModes/MP_GG_GM.GunList` _asmp_gg_gm))
  (if (>= _gungameindex (`KismetArrayLibrary.Array_Length` _gunlist))
    (`/Engine/EditorBlueprintResources/ActorMacros.Switch Has Authority`
      (:`Authority`
        (bind _asmp_gg_gm_2 (cast `/Game/BP/GameModes/MP_GG_GM` (`GameplayStatics.GetGameMode`)))
        (bind _asmain_player_state_bp (cast `/Game/BP/Player/MainPlayerState_BP` (`self.PlayerState`)))
        (`/Game/BP/GameModes/MP_Base_GM.OverrideWin` _asmp_gg_gm_2 (`/Game/BP/Player/MainPlayerState_BP.Name` _asmain_player_state_bp))))
    (else
      (bind _asplayer_bp (cast `/Game/BP/Player/Player_BP` (`self.K2_GetPawn`)))
      (`/Game/BP/Player/Player_BP.Next Weapon` _asplayer_bp (`|GetArrayItem` _gunlist _gungameindex)))))

(fn `UserConstructionScript`)