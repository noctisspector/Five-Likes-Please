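; Lobby player that serves as a smoothly moving viewpoint and sets up the start menu.
; On BeginPlay it takes its target transform from DummyGun_BP camera locations after a short delay, and Tick interpolates location and rotation toward it.
; Unless skipped, it creates the start menu with UI-only input and a message widget stored in Main_GI, which ResetWidgets can rebuild.
; Any key press is recorded as LastKey in the game instance.
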(event `Init Camera`
  (`KismetSystemLibrary.Delay` 0.2)
  (bind _outactors (`GameplayStatics.GetAllActorsOfClass` "/Game/BP/DummyGun_BP.DummyGun_BP_C"))
  (for _array_element _outactors
    (bind _transform (`/Game/BP/DummyGun_BP.GetCameraLocation` _array_element 0 true))
    (`self.UpdateDesiredLocation` _transform)))

(event `Reset Widgets`
  (bind _returnvalue (`GameplayStatics.GetPlayerController` 0))
  (`WidgetLayoutLibrary.RemoveAllWidgets`)
  (bind _returnvalue_2 (`|CreateWidget` "/Game/BP/UI/MainMenu/StartMenu_BP.StartMenu_BP_C" _returnvalue :!label _label))
  (`UserWidget.AddToViewport` _returnvalue_2 0)
  (bind _output_get (set `self.Start Menu` _returnvalue_2))
  (set `PlayerController.bShowMouseCursor` true (`Widget.GetOwningPlayer` _returnvalue_2))
  (`WidgetBlueprintLibrary.SetInputMode_UIOnlyEx` _returnvalue _output_get)
  (bind _returnvalue_3 (`|CreateWidget` "/Game/BP/UI/MessageWidget_BP.MessageWidget_BP_C" _returnvalue))
  (`UserWidget.AddToViewport` _returnvalue_3 0)
  (set `/Game/BP/Main_GI.MessageWidget` _returnvalue_3 (cast `/Game/BP/Main_GI` (`GameplayStatics.GetGameInstance`) :!pure true)))

(event `self.ReceiveBeginPlay`
  (set `self.DesiredTransform` (`self.GetTransform`))
  (`self.Init Camera`)
  (if (not (`self.bSkipWidget`))
    (goto _label)))

(event `Key|AnyKey`
  (params (Key :type "Key Structure"))
  (:`Pressed`
    (set `/Game/BP/Main_GI.LastKey` Key (`self.GI`))))

(event `self.ReceiveTick`
  (params (DeltaSeconds :type "Float (single-precision)"))
  (bind (_desiredtransform_location _desiredtransform_rotation) (`KismetMathLibrary.BreakTransform` (`self.DesiredTransform`)))
  (bind _movespeed (`self.MoveSpeed`))
  (`self.K2_SetActorLocationAndRotation` (`KismetMathLibrary.VInterpTo` (`self.K2_GetActorLocation`) _desiredtransform_location DeltaSeconds _movespeed) (`KismetMathLibrary.RInterpTo` (`self.K2_GetActorRotation`) _desiredtransform_rotation DeltaSeconds _movespeed)))

(fn `UpdateDesiredLocation`
  (params (DesiredTransform :type "Transform Structure"))
  (set `self.DesiredTransform` DesiredTransform))

(fn `UserConstructionScript`)