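; Player state for the main multiplayer player, holding name, team, score and likes, and relaying next-jug requests to the MP_JUG_GM game mode.
; Tick waits for a valid pawn, then once caches its controller and, for the local player, sets the GameInstance name through the server.
; On authority, BeginPlay and GameTick get the team from the game mode.
; Helpers adjust local score and likes, with like removal routed through a server event.
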(event `self.ReceiveTick`
  (params (DeltaSeconds :type "Float (single-precision)"))
  (bind _pawnprivate (`self.PawnPrivate`))
  ;[1 1 1] Get Controller
  (`/Engine/EditorBlueprintResources/StandardMacros.IsValid` _pawnprivate
    (:`Is Valid`
      (`/Engine/EditorBlueprintResources/StandardMacros.DoOnce` false
        (:`Completed`
          (set `self.Controller` (`Pawn.GetController` _pawnprivate))
          ;[1 1 1] Set Name
          (if (== (`GameplayStatics.GetPlayerController` 0) (`self.Controller`))
            (`self.Set Name` (`/Game/BP/Main_GI.Player Name` (`self.GI`)))))))))

(event `Set Name`
  (params (Name :type String))
  ;[1 1 1] Set Name
  (`/Engine/EditorBlueprintResources/ActorMacros.Switch Has Authority`
    (:`Authority`
      (set `self.Name` Name))
    (:`Remote`
      (`self.Set Name Server` Name))))

(event `Set Name Server`
  (params (Name :type String))
  ;[1 1 1] Set Name
  (set `self.Name` Name))

(event `self.ReceiveBeginPlay`
  (`|ExecutionSequence`
    (:`then_1`
      ;[1 1 1] Team Assignment
      (`/Engine/EditorBlueprintResources/ActorMacros.Switch Has Authority` :!label _label
        (:`Authority`
          (bind _team (`/Game/BP/GameModes/MP_Base_GM.Team Assign` (`self.Gamemode`) self))
          (set `self.Team` _team))))))

(event `Team Assign`
  ;[1 1 1] Team Assignment
  (goto _label))

(event `Game Tick`
  (`self.Team Assign`))

(event `Remove Likes toServer`
  (params (` ` :type Integer))
  (`self.Remove Likes Server` ` `))

(event `Remove Likes Server`
  (params (` ` :type Integer))
  (`self.Add Likes` (* ` ` -1)))

(fn `Add Likes`
  (params (`  ` :type Integer))
  (set `self.Local Likes` (+ `  ` (`self.Local Likes`))))

(fn `Add Score`
  (params (`  ` :type "Float (double-precision)"))
  (set `self.Local Score` (+ (`self.Local Score`) `  `)))

(fn `Next Jug`
  (bind _asmp_jug_gm (cast `/Game/BP/GameModes/MP_JUG_GM` (`self.Gamemode`)))
  (`/Game/BP/GameModes/MP_JUG_GM.Find Next Jug` _asmp_jug_gm))

(fn `UserConstructionScript`)