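; Kill cam camera that shows a player the instigator (Inst), presumably their killer, after a death.
; On possession it reads Inst's class, name and, for Player_BP, gun loadout, then HUDClient passes them with the killcam timer to a KillCamUI_BP widget.
; Tick smoothly turns the camera toward Inst with look-at interpolation on pitch and yaw.
; KillReplay removes the widget and destroys the actor.
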(event `HUD Client`
  (bind _returnvalue (`GameplayStatics.GetPlayerController` 0))
  (bind _inst_name (`self.Inst Name`))
  ;[1 1 1] Init HUD
  (bind _returnvalue_2 (`|CreateWidget` "/Game/BP/UI/Ingame/KillCamUI_BP.KillCamUI_BP_C" _returnvalue))
  (`UserWidget.AddToViewport` _returnvalue_2 0)
  (set `self.HUD` _returnvalue_2)
  (`/Game/BP/UI/Ingame/KillCamUI_BP.Init` _returnvalue_2 (`self.Inst Class`) (`self.Inst Loadout`) _inst_name (`/Game/BP/Player/PlayerControllerGame_BP.Killcam Timer` (cast `/Game/BP/Player/PlayerControllerGame_BP` _returnvalue :!pure true)) (not (`KismetStringLibrary.EqualEqual_StrStr` _inst_name))))

(event `self.ReceiveBeginPlay`
  ;[1 1 1] Init HUD
)

(event `self.ReceivePossessed`
  (params (NewController :type "Controller Object Reference"))
  (bind _inst (`self.Inst`))
  ;[1 1 1] Init HUD
  (set `self.Valid Inst` (`KismetSystemLibrary.IsValid` _inst))
  (set `self.Inst Class` (`GameplayStatics.GetObjectClass` _inst))
  (bind _asplayer_bp (cast `/Game/BP/Player/Player_BP` _inst)
    (:`then`
      (set `self.Inst Loadout` (`/Game/BP/Player/Player_BP.GunInit` _asplayer_bp)))
    (:`CastFailed`
      _))
  (set `self.Inst Name` (`/Game/BP/Player/MainPlayerState_BP.Name` (cast `/Game/BP/Player/MainPlayerState_BP` (`Pawn.PlayerState` _inst) :!pure true)))
  (`self.HUD Client`))

(event `Kill Replay`
  ;[1 1 1] Kill
  (`Widget.RemoveFromParent` (`self.HUD`))
  (`self.K2_DestroyActor`))

(event `self.ReceiveTick`
  (params (DeltaSeconds :type "Float (single-precision)"))
  (bind _camera (`self.Camera`))
  ;[1 1 1] Rotate to player
  (bind _output_get (set `self.Inst Location` (`self.K2_GetActorLocation` (`self.Inst`))))
  (bind (_returnvalue_roll _returnvalue_pitch _returnvalue_yaw) (`KismetMathLibrary.BreakRotator` (`KismetMathLibrary.FindLookAtRotation` (`self.K2_GetActorLocation`) _output_get)))
  (`SceneComponent.K2_SetWorldRotation` _camera (`KismetMathLibrary.RInterpTo` (`SceneComponent.K2_GetComponentRotation` _camera) (`KismetMathLibrary.MakeRotator` 0.0 _returnvalue_pitch _returnvalue_yaw) DeltaSeconds 5.0) false false))

(fn `UserConstructionScript`)