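; DummyGun_BP is a preview actor that displays the player's selected gun with its loadout.
; On BeginPlay it sets a child actor to the gun class from Main_GI and calls SetupGun in dummy mode with saved attachments, camo and skin.
; UpdateGunPreview refreshes by spawning a replacement copy, re-running setup on it and destroying itself.
; GetCameraLocation returns the gun's view transform for an attachment category or the full view.
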(event `self.ReceiveBeginPlay`
  (bind _gun (`self.Gun`))
  (bind _asmain_gi (cast `/Game/BP/Main_GI` (`GameplayStatics.GetGameInstance`) :!pure true))
  (bind (_muzzle _underbarrel _sidebarrel _barrel _stock _sight _ammo _camo _equiptment _playerskin) (break `/Game/BP/Player/GunLoadout` (`/Game/BP/Main_GI.Gun Loadout` _asmain_gi)))
  (`ChildActorComponent.SetChildActorClass` _gun (`/Game/BP/Main_GI.Gun` _asmain_gi) :!label _label)
  (`/Game/BP/Weapons/Gun_BP.Setup Gun` (cast `/Game/BP/Weapons/Gun_BP` (`ChildActorComponent.ChildActor` _gun) :!pure true) (make `/Game/BP/Player/GunLoadout` (`self.Test for Attachment` _muzzle) (`self.Test for Attachment` _underbarrel) (`self.Test for Attachment` _sidebarrel) (`self.Test for Attachment` _barrel) (`self.Test for Attachment` _stock) (`self.Test for Attachment` _sight) (`self.Test for Attachment` _ammo) (`/Game/BP/Main_GI.Camo` _asmain_gi) _ _playerskin) true))

(event `Init2`
  (goto _label))

(event `UpdateGunPreview`
  (bind _returnvalue (`|SpawnActorFromClass` "DummyGun_BP_C" (`self.GetTransform`) "AlwaysSpawn" "OverrideRootScale" null null))
  (bind _output_get (set `self.New Dummy` _returnvalue))
  (`ChildActorComponent.SetChildActorClass` (`/BP/DummyGun_BP.Gun` _output_get) (`/Game/BP/Main_GI.Gun` (cast `/Game/BP/Main_GI` (`GameplayStatics.GetGameInstance`) :!pure true)))
  (`self.Init2` _output_get)
  (`self.K2_DestroyActor`))

(fn `GetCameraLocation`
  (params (Category :type Integer) (bFull :type Boolean))
  (returns (Transform :type "Transform Structure"))
  (bind _asgun_bp (cast `/Game/BP/Weapons/Gun_BP` (`ChildActorComponent.ChildActor` (`self.Gun`)) :!pure true))
  (bind _viewmain (`/Game/BP/Weapons/Gun_BP.ViewMain` _asgun_bp))
  (return (`SceneComponent.K2_GetComponentToWorld` (select `bool` bFull :`false` (select `int` Category :`0` (`/Game/BP/Weapons/Gun_BP.ViewMuzzle` _asgun_bp) :`1` (`/Game/BP/Weapons/Gun_BP.ViewUnderbarrel` _asgun_bp) :`2` (`/Game/BP/Weapons/Gun_BP.ViewSideBarrel` _asgun_bp) :`3` (`/Game/BP/Weapons/Gun_BP.ViewBarrel` _asgun_bp) :`4` (`/Game/BP/Weapons/Gun_BP.ViewStock` _asgun_bp) :`5` (`/Game/BP/Weapons/Gun_BP.ViewSight` _asgun_bp) :`6` _viewmain) :`true` _viewmain))))

(fn `UserConstructionScript`)