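; Rifle scope weapon attachment, a child Blueprint that loads its stats from the RifleScope row of the attachment data table.
; On BeginPlay it creates a dynamic cover material on the scope glint and feeds it the aim alpha every tick.
; When the game instance has low scopes enabled, it hides the render target, swaps in a plain scope material and destroys the scope capture component to save cost.
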(event `self.ReceiveBeginPlay`
  (`parent.ReceiveBeginPlay`)
  (bind _returnvalue (`PrimitiveComponent.CreateDynamicMaterialInstance` (`self.ScopeGlint`) 0 "/Game/Material/Scope/ScopeCover_MI.ScopeCover_MI" "None"))
  (set `self.ScopeOuter` _returnvalue)
  (if (`/Game/BP/Main_GI.bLowScopes` (cast `/Game/BP/Main_GI` (`GameplayStatics.GetGameInstance`) :!pure true))
    (`self.Remove LOD`)))

(event `self.ReceiveTick`
  (params (DeltaSeconds :type "Float (single-precision)"))
  (`parent.ReceiveTick` DeltaSeconds)
  (`MaterialInstanceDynamic.SetScalarParameterValue` (`self.ScopeOuter`) "Aim Alpha" (`self.Aim Alpha`)))

(fn `Remove LOD`
  (bind _render_target (`self.Render Target`))
  (`parent.Remove LOD`)
  (`SceneComponent.SetVisibility` _render_target false false)
  (`PrimitiveComponent.SetMaterial` _render_target 0 "/Game/Material/Diffuse/Scope_M.Scope_M")
  (`self.TryDest` (`self.Scope Capture`)))

(fn `Table Stats`
  (returns (` ` :type "/Game/BP/Weapons/Attachment_Stats Structure"))
  (bind _returnvalue (`|GetDataTableRow` "/Game/BP/Weapons/Attachment_Table.Attachment_Table" "RifleScope")
    (:`then`
      (bind _output_get (set `self.Attachment Stats` _returnvalue))
      (return _output_get))))

(fn `UserConstructionScript`
  (`parent.UserConstructionScript`))