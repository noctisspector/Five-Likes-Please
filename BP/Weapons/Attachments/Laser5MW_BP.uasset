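; Weapon attachment Blueprint for the 5MW laser, a child class that specializes a parent attachment with a SpotLight.
; Table Stats fills AttachmentStats from the Laser_5MW row of the attachment data table.
; Overrides of Remove LOD and Set Camo Colors call the parent, then zero the spotlight's intensity or recolor it from the camo color.
; The event graph holds only disabled stubs.
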(fn `Remove LOD`
  (`parent.Remove LOD`)
  (`LightComponent.SetIntensity` (`self.SpotLight`) 0.0))

(fn `Set Camo Colors`
  (params (` ` :type "Color Structure") (`  ` :type "MaterialInstance Object Reference"))
  (`parent.Set Camo Colors` ` ` `  `)
  (`LightComponent.SetLightColor` (`self.SpotLight`) (`KismetMathLibrary.Conv_ColorToLinearColor` ` `) true))

(fn `Table Stats`
  (returns (` ` :type "/Game/BP/Weapons/Attachment_Stats Structure"))
  (bind _returnvalue (`|GetDataTableRow` "/Game/BP/Weapons/Attachment_Table.Attachment_Table" "Laser_5MW")
    (:`then`
      (bind _output_get (set `self.Attachment Stats` _returnvalue))
      (return _output_get))))

(fn `UserConstructionScript`
  (`parent.UserConstructionScript`))