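; XM scope weapon attachment Blueprint with a built-in rangefinder, loading its stats from the XM_SCOPE row of the attachment data table.
; Each tick it line-traces forward from its Tracer component, ignoring player actors, and writes the hit distance to the Range of its XMreader widget.
; GetDist reruns the trace to store and return a set distance on that widget.
; Its spotlight takes its color from the camo colors and switches off in RemoveLOD.
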(event `self.ReceiveTick`
  (params (DeltaSeconds :type "Float (single-precision)"))
  (`parent.ReceiveTick` DeltaSeconds)
  (bind (_bblockinghit _distance) (`self.Trace`))
  (if _bblockinghit
    (bind _asxmreader_bp (cast `/Game/BP/UI/XMreader_BP` (`WidgetComponent.GetUserWidgetObject` (`self.Widget`))))
    (set `/Game/BP/UI/XMreader_BP.Range` _distance _asxmreader_bp)))

(fn `Get Dist`
  (returns (Dist :type "Float (double-precision)"))
  (bind (_bblockinghit _distance) (`self.Trace`))
  (if _bblockinghit
    (bind _asxmreader_bp (cast `/Game/BP/UI/XMreader_BP` (`WidgetComponent.GetUserWidgetObject` (`self.Widget`))))
    (bind _output_get (set `/Game/BP/UI/XMreader_BP.Set` _distance _asxmreader_bp))
    (return _output_get)))

(fn `Remove LOD`
  (`parent.Remove LOD`)
  (`LightComponent.SetIntensity` (`self.SpotLight`) 0.0))

(fn `Set Camo Colors`
  (params (` ` :type "Color Structure") (`  ` :type "MaterialInstance Object Reference"))
  (`parent.Set Camo Colors` ` ` `  `)
  (`LightComponent.SetLightColor` (`self.SpotLight`) (`KismetMathLibrary.Conv_ColorToLinearColor` ` `) true))

(fn `Table Stats`
  (returns (` ` :type "/Game/BP/Weapons/Attachment_Stats Structure"))
  (bind _returnvalue (`|GetDataTableRow` "/Game/BP/Weapons/Attachment_Table.Attachment_Table" "XM_SCOPE")
    (:`then`
      (bind _output_get (set `self.Attachment Stats` _returnvalue))
      (return _output_get))))

(fn `Trace`
  (returns (bBlockingHit :type Boolean) (Distance :type "Float (double-precision)"))
  (bind _tracer (`self.Tracer`))
  (bind _returnvalue (`SceneComponent.K2_GetComponentLocation` _tracer))
  (bind _outactors (`GameplayStatics.GetAllActorsOfClass` "/Game/BP/Player/Player_BP.Player_BP_C"))
  (bind _outhit (`KismetSystemLibrary.LineTraceSingle` _returnvalue (+ _returnvalue (`KismetMathLibrary.GreaterGreater_VectorRotator` (100000000.0 0.0 0.0) (`SceneComponent.K2_GetComponentRotation` _tracer))) "TraceTypeQuery2" true _outactors))
  (bind (_bblockinghit _binitialoverlap _time _distance) (`GameplayStatics.BreakHitResult` _outhit))
  (return _bblockinghit _distance))

(fn `UserConstructionScript`
  (`parent.UserConstructionScript`))