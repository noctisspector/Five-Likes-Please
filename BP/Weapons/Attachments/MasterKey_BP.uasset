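; MasterKey weapon attachment that carries its own fireable gun, a MasterKeyWeapon_BP held in the Weapon child actor.
; Init stores the camo and owning player, passes the player to that gun and sets it up with the camo and a fixed player skin.
; Shoot press and release are forwarded to the inner gun's fire functions, while attachment stats come from the MasterKey row of Attachment_Table.
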(fn `InitMasterKey`
  (params (Camo :type "MaterialInstance Object Reference") (`Player Parent` :type "/Game/BP/Player/PlayerParent_BP Object Reference"))
  (bind __ (`self.Gun`))
  (set `self.Camo` Camo)
  (set `self.Player Parent` `Player Parent`)
  (set `/Game/BP/Weapons/Gun_BP.AttachmentPlayerParent` (`self.Player Parent`) __)
  (`/Game/BP/Weapons/Gun_BP.Setup Gun` __ (make `/Game/BP/Player/GunLoadout` null null null null null null null (`self.Camo`) _ "Soldier1") false))

(fn `Pressing Shoot`
  (params (`Spawn Proj` :type Boolean))
  (`/Game/BP/Weapons/Gun_BP.Press Fire` (`self.Gun`) `Spawn Proj`))

(fn `Releasing Shoot`
  (params (`Spawn Proj` :type Boolean))
  (`/Game/BP/Weapons/Gun_BP.Release Fire` (`self.Gun`) `Spawn Proj`))

(fn `Table Stats`
  (returns (` ` :type "/Game/BP/Weapons/Attachment_Stats Structure"))
  (bind _returnvalue (`|GetDataTableRow` "/Game/BP/Weapons/Attachment_Table.Attachment_Table" "MasterKey")
    (:`then`
      (bind _output_get (set `self.Attachment Stats` _returnvalue))
      (return _output_get))))

(fn `UserConstructionScript`
  (`parent.UserConstructionScript`))