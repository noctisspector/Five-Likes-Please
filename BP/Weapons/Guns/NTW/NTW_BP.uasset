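; Blueprint for the NTW bolt-action gun, a child weapon that supplies its own stats and bolt animation.
; GetTableProperties fills GunStats from the "NTW" row of the gun stats data table.
; PlayBoltAnimation runs the parent behavior, then triggers BoltAnim, which waits BoltDelay before playing the bolt montage on the BOLT component's anim instance.
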(event `Bolt Anim`
  (`KismetSystemLibrary.Delay` (`self.Bolt Delay`))
  (`AnimInstance.Montage_Play` (`SkeletalMeshComponent.GetAnimInstance` (`self.BOLT`)) "/Game/Mesh/Weapons/NTW/ntw_bolt_Anim_Montage.ntw_bolt_Anim_Montage" 1.0 "MontageLength" 0.0 true))

(fn `Get Table Properties`
  (bind _returnvalue (`|GetDataTableRow` "/Game/BP/Weapons/Gun_Stats_Table.Gun_Stats_Table" "NTW")
    (:`then`
      (set `self.Gun Stats` _returnvalue))))

(fn `Play Bolt Animation`
  (`parent.Play Bolt Animation`)
  (`self.Bolt Anim`))

(fn `UserConstructionScript`
  (`parent.UserConstructionScript`))