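; MasterKeyWeapon_BP is the MasterKey gun, a child weapon Blueprint that adds its own stats and a shotgun cocking sound to inherited gun behavior.
; It fills GunStats from the MasterKeyWeapon row of Gun_Stats_Table.
; Its custom fire event runs the parent's fire logic, then calls SoundCustom, which plays the cocking sound at the weapon's location after a short delay.
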(event `SoundCustom`
  (`KismetSystemLibrary.Delay` 0.3)
  (`GameplayStatics.PlaySoundAtLocation` "/Game/Sound/Gun_Sounds_Pro_HD_Remake/Wavs/Cock_Shotgun_4.Cock_Shotgun_4" (`self.K2_GetActorLocation`) (struct) 1.0 1.0 0.0 "/Game/Sound/Human_ATT.Human_ATT" "/Game/Sound/Human_CON.Human_CON" null))

(fn `Custom Fire Event`
  (`parent.Custom Fire Event`)
  (`self.SoundCustom`))

(fn `Get Table Properties`
  (bind _returnvalue (`|GetDataTableRow` "/Game/BP/Weapons/Gun_Stats_Table.Gun_Stats_Table" "MasterKeyWeapon")
    (:`then`
      (set `self.Gun Stats` _returnvalue))))

(fn `UserConstructionScript`
  (`parent.UserConstructionScript`))