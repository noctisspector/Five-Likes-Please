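; RPG weapon Blueprint, a child gun class that specializes its parent's fire and reload behavior for a rocket launcher.
; It reads the "RPG" row from the gun stats data table into GunStats.
; The fire and reload events call their parent versions, then hide the Rocket component on firing and show it again on reload.
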(fn `Custom Fire Event`
  (`parent.Custom Fire Event`)
  (`SceneComponent.SetVisibility` (`self.Rocket`) false false))

(fn `Custom Reload Event`
  (`parent.Custom Reload Event`)
  (`SceneComponent.SetVisibility` (`self.Rocket`) true false))

(fn `Get Table Properties`
  (bind _returnvalue (`|GetDataTableRow` "/Game/BP/Weapons/Gun_Stats_Table.Gun_Stats_Table" "RPG")
    (:`then`
      (set `self.Gun Stats` _returnvalue))))

(fn `UserConstructionScript`
  (`parent.UserConstructionScript`))