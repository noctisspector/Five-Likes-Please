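; Lingering area-damage actor that periodically hurts players near it on behalf of its Thrower, then destroys itself after its lifetime.
; The server alone runs a looping damage timer and the lifetime delay.
; Each tick scans all PlayerParent_BP actors by distance rather than collision, skipping dead players and those passing the Thrower team check.
; Each hit applies damage with a status effect and shows the Thrower a non-kill hitmarker.
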(event `self.ReceiveBeginPlay`
  (`/Engine/EditorBlueprintResources/ActorMacros.Switch Has Authority`
    (:`Authority`
      (`KismetSystemLibrary.K2_SetTimerDelegate` (delegate `Damage Clock`) (`self.Damage Delay`) true)
      (`KismetSystemLibrary.Delay` (`self.Lifetime`))
      (`self.K2_DestroyActor`))))

(event `Damage Clock`
  (bind _thrower (`self.Thrower`))
  (bind _outactors (`GameplayStatics.GetAllActorsOfClass` "/Game/BP/Player/PlayerParent_BP.PlayerParent_BP_C"))
  (for _array_element _outactors
    (bind __ (`/Game/BP/Player/PlayerParent_BP.(P) Check Team` _array_element _thrower))
    (if __
      _
      (elif (`/Game/BP/Player/PlayerParent_BP.bDead` _array_element)
        _
        (elif (< (`self.GetDistanceTo` _array_element) (`self.Radius`))
          (`/Game/BP/Player/PlayerParent_BP.ModifyHealth` _array_element (* (`self.Damage`) -1.0) _thrower (0.0 0.0 0.0) false false "NewEnumerator3" false false 0.0)
          (`/Game/BP/Player/PlayerParent_BP.Hitmarker` _thrower false false ""))))))

(fn `UserConstructionScript`)