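; Configurable weapon projectile for bullets and explosives that damages players and target dummies, with options for sticking, delayed, instant or max-range detonation.
; Overlaps, timers and range checks feed an impact chain that spawns effects and decals and applies distance-scaled, headshot and vehicle-multiplied damage.
; Server-side area damage uses line-of-sight traces, team checks and falloff curves, optionally spawning lingering effects.
; FMJ rounds survive impacts with reduced damage; others are destroyed.
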(event `self.ReceiveHit`
  (params (MyComp :type "PrimitiveComponent Object Reference") (Other :type "Actor Object Reference") (OtherComp :type "PrimitiveComponent Object Reference") (bSelfMoved :type Boolean) (HitLocation :type "Vector Structure") (HitNormal :type "Vector Structure") (NormalImpulse :type "Vector Structure") (Hit :type "HitResult Structure (by ref)"))
  ;[1 1 1] EXP Delay
  (`/Engine/EditorBlueprintResources/StandardMacros.DoOnce` false :!label _label
    (:`Completed`
      (`self.Has Exp Delay`
        (:`true`
          (`/Engine/EditorBlueprintResources/ActorMacros.Switch Has Authority`
            (:`Authority`
              (`self.ExpDelayEvent Local`))))))))

(event `self.ReceiveBeginPlay`
  ;[1 1 1] Init
  (set `self.Initial Location` (`self.K2_GetActorLocation`))
  (set `self.Initial Rotation` (`self.K2_GetActorRotation`))
  (`|ExecutionSequence`
    (:`then_0`
      (`self.Has Exp Delay`
        (:`true`
          (if (`self.bStick`)
            (goto _label)))
        (:`false`
          (`KismetSystemLibrary.Delay` 10.0)
          (`self.K2_DestroyActor`))))
    (:`then_1`
      (if (`self.binstant`)
        (`/Engine/EditorBlueprintResources/ActorMacros.Switch Has Authority`
          (:`Authority`
            (`self.Try Impact` null (`self.K2_GetActorLocation`) (1.0 0.0 0.0))))))))

(event `self.ReceiveTick`
  (params (DeltaSeconds :type "Float (single-precision)"))
  ;[1 1 1] XM EXP
  (if (`self.bXM`)
    (if (>= (`KismetMathLibrary.Vector_Distance` (`self.Initial Location`) (`self.K2_GetActorLocation`)) (`self.XMRange`))
      (`/Engine/EditorBlueprintResources/StandardMacros.DoOnce` false
        (:`Completed`
          (`self.Try Impact` null (`self.K2_GetActorLocation`)))))))

(event `Edit Velocity`
  (params (` ` :type "Float (double-precision)") (ProjectileGravityScale :type "Float (double-precision)"))
  (bind _projectilemovement (`self.ProjectileMovement`))
  ;[1 1 1] Replicate Velocity
  (set `MovementComponent.Velocity` (* (`MovementComponent.Velocity` _projectilemovement) ` `) _projectilemovement)
  (set `ProjectileMovementComponent.ProjectileGravityScale` ProjectileGravityScale _projectilemovement))

(event `Try Impact`
  (params (Object :type "Object Object Reference") (Impact :type "Vector Structure") (Normal :type "Vector Structure"))
  (bind (_returnvalue_x _returnvalue_y _returnvalue_z) (`KismetMathLibrary.BreakVector` (`self.K2_GetActorLocation`)))
  (bind (_asplayer_bp _bsuccess) (`self.Try Get Player`))
  (bind _headshot_mp (`self.Headshot MP`))
  (bind _impact (`self.Impact`))
  (bind _normal (`self.Normal`))
  (bind _firing_actor (`self.Firing Actor`))
  (bind _damage_radius (`self.Damage Radius`))
  (bind _firing_actor_2 (`self.Firing Actor`))
  (bind _damage_curve (`self.Damage Curve`))
  (bind _firing_pawn (`self.Firing Pawn`))
  (bind _player (`self.Player`))
  (bind _vehiclemultiplier (`self.VehicleMultiplier`))
  (bind _bveh (`self.bVeh`))
  (bind _firing_actor_3 (`self.Firing Actor`))
  (bind _impact_2 (`self.Impact`))
  (bind _bullseye (`/Game/BP/Environment/TargetPreview_BP.HitBullseye` (`self.target`) (`self.Impact`)))
  (bind _returnvalue (select `bool` (`self.bExpDelay`) :`false` (`self.Impact`) :`true` (`self.K2_GetActorLocation`)))
  (bind (_returnvalue_x_2 _returnvalue_y_2 _returnvalue_z_2) (`KismetMathLibrary.BreakVector` (`SceneComponent.K2_GetComponentLocation` (`/Game/BP/Player/Player_BP.Headshot Threshold` _asplayer_bp))))
  (bind _returnvalue_2 (select `bool` _bsuccess :`true` (> _returnvalue_z _returnvalue_z_2)))
  (bind _returnvalue_3 (* (select `bool` (`KismetSystemLibrary.IsValid` _damage_curve) :`false` 1.0 :`true` (`CurveFloat.GetFloatValue` _damage_curve (/ (`KismetMathLibrary.Vector_Distance` (`self.Initial Location`) (`self.K2_GetActorLocation`)) (`self.Base Distance`)))) (`self.Base Damage`)))
  ;[1 1 1] Impact
  (set `self.Impact` Impact)
  (set `self.Normal` Normal)
  (bind _output_get (set `self.Object` Object))
  (message `/Game/BP/Environment/DestructInterface.Destroy` _output_get)
  ;;[1 1 1] Valid Object
  (if (not (`KismetArrayLibrary.Array_Contains` (`self.IgnoredActors`) (`GameplayStatics.GetObjectClass` _output_get)))
    (`/Engine/EditorBlueprintResources/StandardMacros.IsValid` _firing_actor_3
      (:`Is Valid`
        (if (not (== _output_get _firing_actor_3))
          (cast `/BP/Weapons/Projectiles/Projectile_BP` _output_get :!label _label_2
            (:`CastFailed`
              ;;[1 1 1] Spawn Emitter
              (bind _asplayer_parent_bp (cast `/Game/BP/Player/PlayerParent_BP` (`self.Object`))
                (:`then`
                  (set `self.Player` _asplayer_parent_bp)
                  (`self.Spawn Emitter` _impact _normal "/Game/BP/Weapons/Exp/BloodExp_BP.BloodExp_BP_C")
                  (set `self.bHitPlayer` true)
                  ;;[1 1 1] Validate Target
                  (if (`self.bHit`)
                    ;;[1 1 1] Bullet Hole
                    (`self.Decal` (select `bool` (`self.bExpDelay`) :`false` (`self.Impact`) :`true` (`self.K2_GetActorLocation`)) (`self.Normal`) (`self.BulletHoleClass`) (1.0 1.0 1.0) :!label _label_3)
                    (bind _astarget_preview_bp (cast `/Game/BP/Environment/TargetPreview_BP` (`self.object`))
                      (:`then`
                        (set `self.bHasTarget` true)
                        (set `self.target` _astarget_preview_bp)
                        (`/Game/BP/Environment/TargetPreview_BP.Hit Target` _astarget_preview_bp (+ (`self.Exp Damage`) (* (select `bool` _bullseye :`false` 1.0 :`true` _headshot_mp) _returnvalue_3 (select `bool` _bveh :`false` 1.0 :`true` (select `/Game/BP/Player/Scorestreaks/VehicleClass` (`/Game/BP/Environment/TargetPreview_BP.VehicleType` (`self.target`)) :`NewEnumerator0` 1.0 :`NewEnumerator1` _vehiclemultiplier :`NewEnumerator2` _vehiclemultiplier)))))
                        (`/Game/BP/Player/Player_BP.Hitmarker` _firing_actor_2 false _bullseye ""))
                      (:`CastFailed`
                        _))
                    (else
                      (set `self.bHit` true)
                      (`/Engine/EditorBlueprintResources/StandardMacros.IsValid` (`self.Firing Actor`)
                        (:`Is Valid`
                          (bind __ (`/Game/BP/Player/PlayerParent_BP.(P) Check Team` (`self.Firing Actor`) _player))
                          (if (not (or __ (`/Game/BP/Player/PlayerParent_BP.bDead` _player)))
                            ;;[1 1 1] Point Damage
                            (`/Engine/EditorBlueprintResources/ActorMacros.Switch Has Authority`
                              (:`Authority`
                                (`/Game/BP/Player/Player_BP.ModifyHealth` (`self.Player`) (* (select `bool` _returnvalue_2 :`false` 1.0 :`true` _headshot_mp) -1.0 _returnvalue_3 (select `bool` _bveh :`false` 1.0 :`true` (select `/Game/BP/Player/Scorestreaks/VehicleClass` (`/Game/BP/Player/PlayerParent_BP.VehicleType` (`self.Player`)) :`NewEnumerator0` 1.0 :`NewEnumerator1` _vehiclemultiplier :`NewEnumerator2` _vehiclemultiplier))) _firing_actor_2 (* (`self.Normal`) (* (`self.Impact Force`) 50000.0 -1.0)) true false "NewEnumerator0" false _returnvalue_2 (`self.Shot Delay`))
                                ;;[1 1 1] Hitmarker
                                (`/Game/BP/Player/Player_BP.Hitmarker` _firing_actor_2 false _returnvalue_2 "")
                                (if (`.ReturnValue` (`self.Blood Location`))
                                  _
                                  (else
                                    _)))
                              (:`Remote`
                                _))))))))
                (:`CastFailed`
                  (`self.Spawn Emitter` (select `bool` (stale `Exp Multi` _output_get) :`false` _impact :`true` (`self.K2_GetActorLocation`)) _normal (`self.EXP CLASS`) true)
                  (goto _label_3)))
              ;;[1 1 1] Area Damage
              (if (and (> (`self.Damage Radius`) 0.0) (not (`self.bHitArea`)))
                (set `self.bHitArea` true)
                (`/Engine/EditorBlueprintResources/ActorMacros.Switch Has Authority`
                  (:`Authority`
                    (bind _outactors (`GameplayStatics.GetAllActorsOfClass` "/Game/BP/Player/PlayerParent_BP.PlayerParent_BP_C"))
                    (`|ExecutionSequence`
                      (:`then_0`
                        (for _array_element _outactors
                          (bind _returnvalue_4 (`self.K2_GetActorLocation` _array_element))
                          (bind _hit (`self.Check Trace` _returnvalue _returnvalue_4))
                          (if _hit
                            (if (`self.bSkipEXPtracing`)
                              (bind _returnvalue_5 (`KismetMathLibrary.Vector_Distance` _returnvalue_4 _returnvalue))
                              (if (< _returnvalue_5 _damage_radius) :!label _label_4
                                (if (not (`/Game/BP/Player/PlayerParent_BP.bDead` _array_element))
                                  (bind ___2 (`/Game/BP/Player/PlayerParent_BP.(P) Check Team` (`self.Firing Actor`) _array_element))
                                  (if (not ___2)
                                    (`/Game/BP/Player/Player_BP.ModifyHealth` _array_element (* (`CurveFloat.GetFloatValue` (`self.Falloff Curve`) (/ _returnvalue_5 _damage_radius)) (`self.Exp Damage`) -1.0) _firing_actor (0.0 0.0 0.0) true false (`self.StatusEffect`) false false 0.0)
                                    (`/Game/BP/Player/Player_BP.Hitmarker` _firing_actor false false "")))))
                            (else
                              (goto _label_4))))
                        (`self.Play EXP Sound Client` :!label _label_5)
                        (if (`self.bFMJ`)
                          (set `self.Base Damage` (* (`self.Base Damage`) (`self.FMJ_DamagePercent`)))
                          (if (`self.bHitPlayer`)
                            (`KismetSystemLibrary.Delay` 0.1)
                            (set `self.bHit` true))
                          (else
                            (`self.K2_DestroyActor`))))
                      (:`then_1`
                        ;[1 1 1] Linger
                        (if (`self.bLingering`)
                          (bind (_outhit _returnvalue_6) (`KismetSystemLibrary.LineTraceSingle` _impact_2 (- _impact_2 (0.0 0.0 700.0)) "TraceTypeQuery1"))
                          (`|SpawnActorFromClass` (`self.LingerEffect`) (`KismetMathLibrary.MakeTransform` (select `bool` (> (`self.Exp Delay`) 0.0) :`false` (select `bool` (`self.bLingerStatic`) :`false` (select `bool` _returnvalue_6 :`false` _impact_2 :`true` (`.ImpactPoint` (`GameplayStatics.BreakHitResult` _outhit))) :`true` _impact_2) :`true` (`self.K2_GetActorLocation`))) "AlwaysSpawn" "OverrideRootScale" null (`self.Exp Damage`) (`self.Damage Radius`) (`self.Firing Actor`) null)))))
                  (:`Remote`
                    (goto _label_5)))
                (else
                  (goto _label_5)))))))
      (:`Is Not Valid`
        (`/Engine/EditorBlueprintResources/StandardMacros.IsValid` _firing_pawn
          (:`Is Valid`
            (if (not (== _output_get _firing_pawn))
              (goto _label_2)))
          (:`Is Not Valid`
            (goto _label_2)))))))

(event `self.Collision.OnComponentBeginOverlap`
  (params (OverlappedComponent :type "PrimitiveComponent Object Reference") (OtherActor :type "Actor Object Reference") (OtherComp :type "PrimitiveComponent Object Reference") (OtherBodyIndex :type Integer) (bFromSweep :type Boolean) (SweepResult :type "HitResult Structure (by ref)"))
  ;[1 1 1] Overlap
  (if (== (`GameplayStatics.GetObjectClass` OtherActor) "/Game/BP/Game/Hardpoint_BP.Hardpoint_BP_C")
    _
    (elif (`self.bStick`)
      (if (not (`self.bStuck`))
        (set `self.STICK IMPACT` SweepResult_ImpactPoint)
        (set `self.bStuck` true)
        (`ActorComponent.K2_DestroyComponent` (`self.ProjectileMovement`))
        (`self.Stick Events`)
        (`self.K2_SetActorLocation` (`self.STICK IMPACT`)))
      (else
        (`self.Has Exp Delay`
          (:`false`
            (`/Engine/EditorBlueprintResources/ActorMacros.Switch Has Authority`
              (:`Authority`
                (set `self.Last Normal` SweepResult_Normal)
                (`self.Try Impact` OtherActor SweepResult_ImpactPoint SweepResult_Normal)))))))))

(event `Spawn Emitter`
  (params (Location :type "Vector Structure") (Up :type "Vector Structure") (Class :type "Actor Class Reference") (bPhysics :type Boolean))
  ;[1 1 1] Impact
  ;;[1 1 1] Spawn Emitter
  (if bPhysics
    (bind (_outhit _returnvalue) (`KismetSystemLibrary.LineTraceSingle` (+ Location (* Up 50.0)) (+ Location (* Up -50.0)) "TraceTypeQuery1" true))
    (if (and (`KismetSystemLibrary.IsValid` (`.PhysMat` (`GameplayStatics.BreakHitResult` _outhit))) _returnvalue)
      (`/Game/BP/Main_GI.Spawn Particle Physics` (`self.GI`) Location Up (`.PhysMat` (`GameplayStatics.BreakHitResult` _outhit)) (`self.Impact Type`) (castclass `/Game/BP/Weapons/Exp/EXP_BP` Class :!pure true))
      (else
        (`|SpawnActorFromClass` Class (`KismetMathLibrary.MakeTransform` Location (`KismetMathLibrary.MakeRotationFromAxes` (0.0 0.0 0.0) (0.0 0.0 0.0) Up)) "Undefined" "OverrideRootScale" null null :!label _label_6)))
    (else
      (goto _label_6))))

(event `ExpDelayEvent Local`
  ;[1 1 1] Impact
  (`KismetSystemLibrary.K2_SetTimerDelegate` (delegate `ExpDelay TIMER`) (`self.Exp Delay`)))

(event `ExpDelay TIMER`
  ;[1 1 1] Impact
  (`self.Exp Multi` (`self.EXP CLASS`)))

(event `Exp Multi`
  (params (Class :type "Actor Class Reference"))
  ;[1 1 1] Impact
  (bind _output_get (set `self.bExpDelay` true))
  (`self.Spawn Emitter` (select `bool` _output_get :`false` (`self.Impact`) :`true` (`self.K2_GetActorLocation`)) (`self.Normal`) Class)
  (goto _label_3))

(event `Decal`
  (params (Location :type "Vector Structure") (Normal :type "Vector Structure (by ref)") (Class :type "/Game/BP/Weapons/BulletHoles/BulletHole_BP Class Reference") (`Spawn Transform Scale` :type "Vector Structure"))
  ;[1 1 1] Impact
  ;;[1 1 1] Bullet Hole
  (`|SpawnActorFromClass` Class (`KismetMathLibrary.MakeTransform` Location (select `bool` (`self.bHoleRotationFromDirection`) :`false` (`KismetMathLibrary.MakeRotFromX` Normal) :`true` (`self.K2_GetActorRotation`)) `Spawn Transform Scale`) "Undefined" "OverrideRootScale" null null))

(event `Play EXP Sound Client`
  (bind _exp_sound (`self.Exp Sound`))
  ;[1 1 1] Impact
  (`/Engine/EditorBlueprintResources/StandardMacros.IsValid` _exp_sound
    (:`Is Valid`
      (`GameplayStatics.PlaySoundAtLocation` _exp_sound (`self.K2_GetActorLocation`) (struct) 1.0 1.0 0.0 "/Game/Sound/Exp_ATT.Exp_ATT" "/Game/Sound/Gun_CON.Gun_CON" null))))

(fn `Blood Location`
  (returns (Impact :type "Vector Structure") (Normal :type "Vector Structure") (ReturnValue :type Boolean))
  (bind _impact (`self.Impact`))
  (bind _outactors (`GameplayStatics.GetAllActorsOfClass` "/Game/BP/Player/PlayerParent_BP.PlayerParent_BP_C"))
  (bind (_outhit _returnvalue) (`KismetSystemLibrary.LineTraceSingle` _impact (+ _impact (* (`self.GetActorForwardVector`) (`self.BloodDistance`))) "TraceTypeQuery1" false _outactors))
  (bind (_bblockinghit _binitialoverlap _time _distance _location _impactpoint _normal _impactnormal) (`GameplayStatics.BreakHitResult` _outhit))
  (return _impactpoint _impactnormal _returnvalue))

(fn `Check Trace`
  (params (Start :type "Vector Structure") (End :type "Vector Structure"))
  (returns (Hit :type Boolean))
  (locals (Ignored :type "Array of Actor Object Reference"))
  (bind _outactors (`GameplayStatics.GetAllActorsOfClass` "/Game/BP/Player/Player_BP.Player_BP_C"))
  (bind _output_get (set `local.Ignored` _outactors))
  (bind _outactors_2 (`GameplayStatics.GetAllActorsOfClass` "Projectile_BP_C"))
  (`KismetArrayLibrary.Array_Append` _output_get _outactors_2)
  (bind (_outhit _returnvalue) (`KismetSystemLibrary.LineTraceSingle` Start End "TraceTypeQuery1" true (`local.Ignored`)))
  (return _returnvalue))

(fn `EXP DELAY CALL`)

(fn `Init`
  (params (Speed :type "Float (double-precision)") (ProjectileGravityScale :type "Float (double-precision)"))
  (`self.Edit Velocity` Speed ProjectileGravityScale))

(fn `Stick Events`)

(fn `Try Get Player`
  (returns (`AsPlayer BP` :type "/Game/BP/Player/Player_BP Object Reference") (bSuccess :type Boolean))
  (bind (_asplayer_bp _bsuccess) (cast `/Game/BP/Player/Player_BP` (`self.Player`) :!pure true))
  (return _asplayer_bp _bsuccess))

(fn `UserConstructionScript`)