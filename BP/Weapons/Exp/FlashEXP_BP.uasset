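; FlashEXP_BP is a flash explosion effect actor, apparently for a flash-type weapon.
; On BeginPlay it shows a BlindingCube mesh and raises a PointLight to very high intensity, then after a short Delay hides the cube and turns the light off.
; The overlap and tick events are disabled, and the actor does not destroy itself in this graph.
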(event `self.ReceiveBeginPlay`
  (bind _blindingcube (`self.BlindingCube`))
  (bind _pointlight (`self.PointLight`))
  (`parent.ReceiveBeginPlay`)
  (`SceneComponent.SetVisibility` _blindingcube true false)
  (`LightComponent.SetIntensity` _pointlight 50000.0)
  (`KismetSystemLibrary.Delay` 0.2)
  (`SceneComponent.SetVisibility` _blindingcube false false)
  (`LightComponent.SetIntensity` _pointlight 0.0))

(fn `UserConstructionScript`
  (`parent.UserConstructionScript`))