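; ClaymoreDrop_BP is a deployed claymore that explodes when an opposing player enters its Detection component.
; On overlap, the server ignores the instigator's own PlayerState and any player matched by PCheckTeam against the instigator.
; For a valid target it latches Overlapped, calls EXPClient to spawn the EXP actor at its location, applies Damage through ModifyHealth credited to the instigator, then destroys itself.
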(event `self.Detection.OnComponentBeginOverlap`
  (params (OverlappedComponent :type "PrimitiveComponent Object Reference") (OtherActor :type "Actor Object Reference") (OtherComp :type "PrimitiveComponent Object Reference") (OtherBodyIndex :type Integer) (bFromSweep :type Boolean) (SweepResult :type "HitResult Structure (by ref)"))
  (bind _insti (`self.Insti`))
  (if (not (`self.bOverlapped`))
    (`/Engine/EditorBlueprintResources/ActorMacros.Switch Has Authority`
      (:`Authority`
        (bind _asplayer_bp (cast `/Game/BP/Player/Player_BP` OtherActor))
        (if (not (== (`self.Inst State`) (`Pawn.PlayerState` _asplayer_bp)))
          (bind __ (`/Game/BP/Player/PlayerParent_BP.(P) Check Team` _asplayer_bp _insti))
          (if (not __)
            (set `self.bOverlapped` true)
            (`self.EXP Client`)
            (`/Game/BP/Player/Player_BP.ModifyHealth` _asplayer_bp (`self.Damage`) _insti (0.0 0.0 0.0) false false "NewEnumerator0" false false 0.0)
            (`self.K2_DestroyActor`)))))))

(event `EXP Client`
  (`|SpawnActorFromClass` (`self.EXP`) (`KismetMathLibrary.MakeTransform` (`self.K2_GetActorLocation`)) "AlwaysSpawn" "OverrideRootScale" null null))

(fn `UserConstructionScript`
  (`parent.UserConstructionScript`))