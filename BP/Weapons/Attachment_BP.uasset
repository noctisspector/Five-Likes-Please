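; Weapon attachment Blueprint that holds an attachment's stats and handles camo on its static mesh.
; Stats come from the Default row of Attachment_Table and supply the ProCon data.
; SetCamo applies a slot material, then uses Main_GI's per-material maps to call SetCamoColors and set the light material.
; UpdateAimAlpha zeroes aim alpha when LowScopes is on; SetCamoColors and RemoveLOD are empty stubs.
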(fn `Generate ProCon`
  (returns (` ` :type "Array of /Game/BP/Weapons/ProConStruct Structure"))
  (return (`.ProCon_48_4DBADA974FD90A3B84EFEE9313992DDF` (break `/Game/BP/Weapons/Attachment_Stats` (`self.Attachment Stats`)))))

(fn `Remove LOD`)

(fn `Set Camo`
  (params (MaterialSlotName :type Name) (Material :type "MaterialInterface Object Reference"))
  (bind _asmain_gi (cast `/Game/BP/Main_GI` (`GameplayStatics.GetGameInstance`) :!pure true))
  (`PrimitiveComponent.SetMaterialByName` (`self.StaticMesh`) MaterialSlotName Material)
  (bind _asmaterial_instance (cast `MaterialInstance` Material))
  (bind (_value _returnvalue) (`BlueprintMapLibrary.Map_Find` (`/Game/BP/Main_GI.Camo Colors` _asmain_gi) _asmaterial_instance))
  (if _returnvalue
    (bind (_value_2 _returnvalue_2) (`BlueprintMapLibrary.Map_Find` (`/Game/BP/Main_GI.Camo Light` _asmain_gi) _asmaterial_instance))
    (`self.Set Camo Colors` _value _value_2))
  (if _returnvalue_2
    (`PrimitiveComponent.SetMaterialByName` (`self.StaticMesh`) (`self.Light Name`) _value_2)))

(fn `Set Camo Colors`
  (params (` ` :type "Color Structure") (`  ` :type "MaterialInstance Object Reference")))

(fn `Table Stats`
  (returns (` ` :type "/Game/BP/Weapons/Attachment_Stats Structure"))
  (bind _returnvalue (`|GetDataTableRow` "/Game/BP/Weapons/Attachment_Table.Attachment_Table" "Default")
    (:`then`
      (bind _output_get (set `self.Attachment Stats` _returnvalue))
      (return _output_get))))

(fn `Update Aim Alpha`
  (params (`Aim Alpha` :type "Float (double-precision)"))
  (set `self.Aim Alpha` (select `bool` (`/Game/BP/Main_GI.bLowScopes` (`self.GI`)) :`false` `Aim Alpha`)))

(fn `UserConstructionScript`)