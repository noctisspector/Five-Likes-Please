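; Automatic double sliding door that opens while any PlayerParent_BP actor is nearby.
; Every Tick it fetches all those actors and sets Open if any is closer than the Sphere radius, using distance polling rather than overlap events.
; An interpolated DoorTransition, scaled by DoorScale, slides DoorL and DoorR in opposite directions along local Y.
; An authority switch is left unconnected, so the check has no network gating.
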(event `self.ReceiveTick`
  (params (DeltaSeconds :type "Float (single-precision)"))
  (bind _output_get (set `self.DoorTransition` (`KismetMathLibrary.FInterpTo` (`self.DoorTransition`) (select `bool` (`self.bOpen`) :`true` 1.0 :!type "Float (single-precision)") DeltaSeconds 5.0)))
  (bind _returnvalue (* _output_get (`self.DoorScale`)))
  (`SceneComponent.K2_SetRelativeLocation` (`self.DoorL`) (`KismetMathLibrary.MakeVector` 0.0 _returnvalue) false false)
  (`SceneComponent.K2_SetRelativeLocation` (`self.DoorR`) (`KismetMathLibrary.MakeVector` 0.0 (* _returnvalue -1.0)) false false)
  (bind _outactors (`GameplayStatics.GetAllActorsOfClass` "/Game/BP/Player/PlayerParent_BP.PlayerParent_BP_C"))
  (bind _output_get_2 (set `self.bTestingOpen` false))
  (for _array_element _outactors
    (if (< (`self.GetDistanceTo` _array_element) (`SphereComponent.SphereRadius` (`self.Sphere`)))
      (set `self.bTestingOpen` true)))
  (set `self.bOpen` _output_get_2))

(fn `UserConstructionScript`)