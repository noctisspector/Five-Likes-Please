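; EventDoor_BP is a sliding double door that opens and closes when its ToggleServer event flips the Open flag.
; Each Tick, FInterpTo eases DoorTransition toward open or closed, then offsets DoorL and DoorR along local Y in opposite directions, scaled by DoorScale.
; Overlap and BeginPlay events are unused, so the toggle must be triggered from outside this graph.
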(event `self.ReceiveTick`
  (params (DeltaSeconds :type "Float (single-precision)"))
  (bind _output_get (set `self.DoorTransition` (`KismetMathLibrary.FInterpTo` (`self.DoorTransition`) (select `bool` (`self.bOpen`) :`true` 1.0 :!type "Float (single-precision)") DeltaSeconds 5.0)))
  (bind _returnvalue (* _output_get (`self.DoorScale`)))
  (`SceneComponent.K2_SetRelativeLocation` (`self.DoorL`) (`KismetMathLibrary.MakeVector` 0.0 _returnvalue) false false)
  (`SceneComponent.K2_SetRelativeLocation` (`self.DoorR`) (`KismetMathLibrary.MakeVector` 0.0 (* _returnvalue -1.0)) false false))

(event `ToggleServer`
  (set `self.bOpen` (not (`self.bOpen`))))

(fn `UserConstructionScript`)