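; Environment light Blueprint that flickers a point light by animating its intensity with a timeline.
; The construction script applies the configurable attenuation radius and intensity.
; On BeginPlay it reapplies the radius, sets a timeline play rate from LightRate and caches the starting intensity.
; Each timeline update multiplies that cached intensity by the curve track, so the flicker scales with the configured brightness.
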(event `self.ReceiveBeginPlay`
  (`LocalLightComponent.SetAttenuationRadius` (`self.PointLight`) (`self.Attenuation Radius`))
  (`TimelineComponent.SetPlayRate` (`self.Timeline_0`) (`self.Light Rate`))
  (bind _output_get (set `self.Initial Intensity` (`LightComponentBase.Intensity` (`self.PointLight`))))
  (bind (_direction _newtrack_0) (`Timeline|Timeline_0` :!via `PlayFromStart`)
    (:`Update`
      (`LightComponent.SetIntensity` (`self.PointLight`) (* _newtrack_0 _output_get)))))

(fn `UserConstructionScript`
  (bind _pointlight (`self.PointLight`))
  (`LocalLightComponent.SetAttenuationRadius` _pointlight (`self.Attenuation Radius`))
  (`LightComponent.SetIntensity` _pointlight (`self.Intensity Set`)))