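; Environmental hazard actor that periodically damages players within a set radius.
; On BeginPlay, the authority starts a looping timer that fires the Damage event every Delay seconds.
; Each tick of that timer scans all PlayerParent_BP actors by distance and applies negative BaseDamage through ModifyHealth to those inside Radius.
; The construction script sizes the Sphere to Radius, but damage relies on the distance check rather than overlaps.
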(event `self.ReceiveBeginPlay`
  (`/Engine/EditorBlueprintResources/ActorMacros.Switch Has Authority`
    (:`Authority`
      (`KismetSystemLibrary.K2_SetTimerDelegate` (delegate `Damage`) (`self.Delay`) true))))

(event `Damage`
  (bind _outactors (`GameplayStatics.GetAllActorsOfClass` "/Game/BP/Player/PlayerParent_BP.PlayerParent_BP_C"))
  (for _array_element _outactors
    (if (< (`self.GetDistanceTo` _array_element) (`self.Radius`))
      (`/Game/BP/Player/PlayerParent_BP.ModifyHealth` _array_element (* (`self.Base Damage`) -1.0) null (0.0 0.0 0.0) false false "NewEnumerator0" false false 0.0))))

(fn `UserConstructionScript`
  (`SphereComponent.SetSphereRadius` (`self.Sphere`) (`self.Radius`) true))