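; Crane environment Blueprint that periodically lowers and raises the "Mover" bone of a poseable mesh.
; BeginPlay caches the bone's world location and, on authority only, starts a looping timer that flips the Moved flag every few seconds.
; Tick runs without an authority check, smoothly interpolating the bone between its original position and a point below it according to that flag.
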(event `self.ReceiveBeginPlay`
  (bind _returnvalue (`PoseableMeshComponent.GetBoneLocationByName` (`self.PoseableMesh`) "Mover" "WorldSpace"))
  (set `self.OriginalLocation` _returnvalue)
  (`/Engine/EditorBlueprintResources/ActorMacros.Switch Has Authority`
    (:`Authority`
      (`KismetSystemLibrary.K2_SetTimerDelegate` (delegate `ChangebMoved`) 7.0 true))))

(event `ChangebMoved`
  (set `self.bMoved` (not (`self.bMoved`))))

(event `self.ReceiveTick`
  (params (DeltaSeconds :type "Float (single-precision)"))
  (bind _poseablemesh (`self.PoseableMesh`))
  (bind _originallocation (`self.OriginalLocation`))
  (bind _returnvalue (`PoseableMeshComponent.GetBoneLocationByName` _poseablemesh "Mover" "WorldSpace"))
  (`PoseableMeshComponent.SetBoneLocationByName` _poseablemesh "Mover" (`KismetMathLibrary.VInterpTo` _returnvalue (select `bool` (`self.bMoved`) :`false` _originallocation :`true` (+ _originallocation (0.0 0.0 -800.0))) DeltaSeconds 1.0) "WorldSpace"))

(fn `UserConstructionScript`)