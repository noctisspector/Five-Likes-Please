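; Interactable lever that toggles every EventDoor_BP in the level through each door's ToggleServer.
; Each Tick, it compares its distance to player 0 with DetectionRadius, writes OnLever and itself as Lever onto PlayerParent_BP, and shows an Interact key tip on entering range.
; ToggleLever, not called within this graph, performs the door toggle.
; The construction script sizes the Sphere to DetectionRadius, though detection uses distance rather than overlaps.
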(event `self.ReceiveTick`
  (params (DeltaSeconds :type "Float (single-precision)"))
  (bind _asplayer_parent_bp (cast `/Game/BP/Player/PlayerParent_BP` (`GameplayStatics.GetPlayerCharacter` 0)))
  (bind _output_get (set `self.OnLeverTemp` (`/Game/BP/Player/PlayerParent_BP.bOnLever` _asplayer_parent_bp)))
  (bind _output_get_2 (set `/Game/BP/Player/PlayerParent_BP.bOnLever` (< (`self.GetDistanceTo` _asplayer_parent_bp) (`self.Detection Radius`)) _asplayer_parent_bp))
  (set `/Game/BP/Player/PlayerParent_BP.Lever` self _asplayer_parent_bp)
  (if _output_get_2
    (if (not _output_get)
      (`/Game/BP/Player/PlayerParent_BP.Keytip` _asplayer_parent_bp "toggle door." "Interact"))))

(event `ToggleLever`
  (bind _outactors (`GameplayStatics.GetAllActorsOfClass` "/Game/BP/Environment/EventDoor_BP.EventDoor_BP_C"))
  (for _array_element _outactors
    (`/Game/BP/Environment/EventDoor_BP.ToggleServer` _array_element)))

(fn `UserConstructionScript`
  (`SphereComponent.SetSphereRadius` (`self.Sphere`) (`self.Detection Radius`) true))