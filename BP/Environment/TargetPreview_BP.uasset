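; TargetPreview_BP is a shootable target that displays received damage on the player's HUD as a damage indicator.
; HitTarget truncates the damage to text and passes it to the PlayerParent_BP HUD.
; A Vehicle flag makes the construction script recolor the mesh green and rescale it, and also selects the enum VehicleType returns.
; HitBullseye reports whether a world location lies within BullseyeDist of the Bullseye component.
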(event `Hit Target`
  (params (Damage :type "Float (double-precision)"))
  (bind _asplayer_parent_bp (cast `/Game/BP/Player/PlayerParent_BP` (`GameplayStatics.GetPlayerPawn` 0)))
  (`/Game/BP/UI/Ingame/InGameHUD_BP.Damage Indicator` (`/Game/BP/Player/PlayerParent_BP.HUD` _asplayer_parent_bp) (`KismetTextLibrary.Conv_IntToText` (`KismetMathLibrary.FTrunc` Damage))))

(fn `HitBullseye`
  (params (`World Location` :type "Vector Structure"))
  (returns (Bullseye :type Boolean))
  (return (< (`KismetMathLibrary.Vector_Distance` `World Location` (`SceneComponent.K2_GetComponentLocation` (`self.Bullseye`))) (`self.BullseyeDist`))))

(fn `UserConstructionScript`
  (if (`self.bVehicle`)
    (`PrimitiveComponent.SetMaterial` (`self.StaticMesh`) 2 "/Game/Material/Diffuse/Green_M.Green_M")
    (`SceneComponent.SetRelativeScale3D` (`self.StaticMesh`) (0.2 0.2 0.2))))

(fn `VehicleType`
  (returns (` ` :type "/Game/BP/Player/Scorestreaks/VehicleClass Enum"))
  (return (select `bool` (`self.bVehicle`) :`false` "NewEnumerator0" :`true` "NewEnumerator1" :!type "/Game/BP/Player/Scorestreaks/VehicleClass Enum")))