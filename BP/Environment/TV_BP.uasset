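; TV_BP is a breakable television prop whose screen and lights react when it is destroyed.
; Destroy calls BreakMulticast, which acts only on the first hit and removes the FlickerLight component.
; It then plays the InitialFlicker timeline, whose alpha drives the point light's intensity and, inverted, the screen material's Broken parameter.
; The construction script creates that dynamic material instance on the mesh's second material slot.
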(event `/Game/BP/Environment/DestructInterface.Destroy`
  (`self.Break Multicast`))

(event `Break Multicast`
  (if (not (`self.bHit`))
    (set `self.bHit` true)
    (`ActorComponent.K2_DestroyComponent` (`self.FlickerLight`))
    (bind (_direction _broken_alpha) (`Timeline|Initial Flicker` :!via `PlayFromStart`)
      (:`Update`
        (`MaterialInstanceDynamic.SetScalarParameterValue` (`self.Material Inst`) "Broken" (- 1.0 _broken_alpha))
        (`LightComponent.SetIntensity` (`self.PointLight`) (* _broken_alpha 500.0))))))

(fn `UserConstructionScript`
  (bind _returnvalue (`PrimitiveComponent.CreateDynamicMaterialInstance` (`self.StaticMesh`) 1 (`self.Material`) "None"))
  (set `self.Material Inst` _returnvalue))