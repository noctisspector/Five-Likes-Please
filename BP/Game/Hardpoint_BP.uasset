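; Hardpoint objective actor, a child Blueprint that awards team and player score to players touching it while active.
; On each game-time update it loops through valid TouchingPlayers, scoring their team and pawn through MP_POINT_GM and notifying the pawn.
; Deactivation clears the touching list, and the square marker's visibility follows the active state.
; The construction script scales the detection volume and marker horizontally by Scale.
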(fn `Gametime Update`
  (if (`self.bActive`)
    (`parent.Gametime Update`)
    (for _array_element (`self.Touching Players`)
      (`/Engine/EditorBlueprintResources/StandardMacros.IsValid` _array_element
        (:`Is Valid`
          (bind _asmp_point_gm (cast `/Game/BP/GameModes/MP_POINT_GM` (`GameplayStatics.GetGameMode`)))
          (`/Game/BP/GameModes/MP_Base_GM.Objective Score` _asmp_point_gm (`/Game/BP/Player/MainPlayerState_BP.Team` (cast `/Game/BP/Player/MainPlayerState_BP` (`Pawn.PlayerState` _array_element) :!pure true)))
          (`/Game/BP/GameModes/MP_Base_GM.Add Player Score` _asmp_point_gm _array_element (`/Game/BP/GameModes/MP_Base_GM.Objective Capture Score` _asmp_point_gm) 0)
          (`/Game/BP/Player/Player_BP.Objective Score` _array_element))))))

(fn `OnActiveUpdate`
  (`parent.OnActiveUpdate`)
  (`SceneComponent.SetVisibility` (`self.obj_squaremarker`) (`self.bActive`) true))

(fn `Set Status`
  (params (Active :type Boolean))
  (`parent.Set Status` Active)
  (if (not Active)
    (`KismetArrayLibrary.Array_Clear` (`self.Touching Players`))))

(fn `UserConstructionScript`
  (bind _obj_squaremarker (`self.obj_squaremarker`))
  (bind _scale (`self.Scale`))
  (bind (_relativescale3d_x _relativescale3d_y _relativescale3d_z) (`KismetMathLibrary.BreakVector` (`SceneComponent.RelativeScale3D` _obj_squaremarker)))
  (`parent.UserConstructionScript`)
  (`SceneComponent.SetRelativeScale3D` (`self.Detection`) (`KismetMathLibrary.MakeVector` _scale _scale 1.0))
  (`SceneComponent.SetRelativeScale3D` _obj_squaremarker (`KismetMathLibrary.MakeVector` (* _relativescale3d_x _scale) (* _relativescale3d_y _scale) _relativescale3d_z)))