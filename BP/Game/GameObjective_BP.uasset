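; Base game objective actor that tracks players inside its detection volume and carries a replicated active state.
; On the server, overlaps maintain the TouchingPlayers list and tell each Player_BP whether it overlaps an active objective.
; A looping one-second server timer calls the empty GametimeUpdate hook.
; SetStatus changes Active only under a Game-derived game mode, and its RepNotify calls the empty OnActiveUpdate hook.
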(event `self.ReceiveBeginPlay`
  (`/Engine/EditorBlueprintResources/ActorMacros.Switch Has Authority`
    (:`Authority`
      (`KismetSystemLibrary.K2_SetTimerDelegate` (delegate `Timer`) 1.0 true))))

(event `Timer`
  (`self.Gametime Update`))

(event `self.Detection.OnComponentBeginOverlap`
  (params (OverlappedComponent :type "PrimitiveComponent Object Reference") (OtherActor :type "Actor Object Reference") (OtherComp :type "PrimitiveComponent Object Reference") (OtherBodyIndex :type Integer) (bFromSweep :type Boolean) (SweepResult :type "HitResult Structure (by ref)"))
  (`/Engine/EditorBlueprintResources/ActorMacros.Switch Has Authority`
    (:`Authority`
      (if (== (`GameplayStatics.GetObjectClass` OtherActor) "/Game/BP/Player/Player_BP.Player_BP_C")
        (bind _asplayer_bp (cast `/Game/BP/Player/Player_BP` OtherActor))
        (`/Game/BP/Player/Player_BP.Set Overlapping Objective` _asplayer_bp (`self.bActive`))
        (`KismetArrayLibrary.Array_AddUnique` (`self.Touching Players`) _asplayer_bp)))))

(event `self.Detection.OnComponentEndOverlap`
  (params (OverlappedComponent :type "PrimitiveComponent Object Reference") (OtherActor :type "Actor Object Reference") (OtherComp :type "PrimitiveComponent Object Reference") (OtherBodyIndex :type Integer))
  (`/Engine/EditorBlueprintResources/ActorMacros.Switch Has Authority`
    (:`Authority`
      (if (== (`GameplayStatics.GetObjectClass` OtherActor) "/Game/BP/Player/Player_BP.Player_BP_C")
        (bind _asplayer_bp (cast `/Game/BP/Player/Player_BP` OtherActor))
        (`/Game/BP/Player/Player_BP.Set Overlapping Objective` _asplayer_bp false)
        (`KismetArrayLibrary.Array_RemoveItem` (`self.Touching Players`) _asplayer_bp)))))

(fn `Gametime Update`)

(fn `OnActiveUpdate`)

(fn `OnRep_bActive`
  (`self.OnActiveUpdate`))

(fn `Set Status`
  (params (Active :type Boolean))
  (if (`KismetMathLibrary.ClassIsChildOf` (`GameplayStatics.GetObjectClass` (`GameplayStatics.GetGameMode`)) (`self.Game`))
    (set `self.bActive` Active)))

(fn `UserConstructionScript`)